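; BP_RBShooterPlayerController is the player controller Blueprint for the RBShooter player, used here to bind debug cheats to number keys.
; Key presses call the CheatManager directly to teleport, toggle slow motion, enable the debug camera or enter ghost mode.
; A FlipFlop alternates the slow-motion key between slowed and normal time.
; BeginPlay, Tick and the construction script contain no logic.
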(event EventBeginPlay)

(event EventTick
  (params (DeltaSeconds :type Float%20%28single-precision%29)))

(event Input|KeyboardEvents|4
  (params (Key :type Key%20Structure :default "None"))
  ;[1 1 1] Handle cheats
  (:Pressed
    (Class|CheatManager|Ghost (Variables|Default|GetCheatManager))))

(event Input|KeyboardEvents|1
  (params (Key :type Key%20Structure :default "None"))
  ;[1 1 1] Handle cheats
  (:Pressed
    (Transformation|Teleport (Variables|Default|GetCheatManager))))

(event Input|KeyboardEvents|2
  (params (Key :type Key%20Structure :default "None"))
  (bind _cheatmanager (Variables|Default|GetCheatManager))
  ;[1 1 1] Handle cheats
  (:Pressed
    (Utilities|FlowControl|FlipFlop
      (:A
        (Class|CheatManager|Slomo _cheatmanager 0.1))
      (:B
        (Class|CheatManager|Slomo _cheatmanager 1.0)))))

(event Input|KeyboardEvents|3
  (params (Key :type Key%20Structure :default "None"))
  ;[1 1 1] Handle cheats
  (:Pressed
    (Class|CheatManager|EnableDebugCamera (Variables|Default|GetCheatManager))))

(fn ConstructionScript)