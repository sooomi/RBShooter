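; Player weapon that charges and fires red or blue projectiles, with a held modifier that fires that color's power ability instead.
; CombatPowerManager bomb points set power tiers (magnet projectile, grenade, zap dome) and damage multipliers; firing a power spends that color's points and briefly disables fire.
; Projectiles aim from muzzle sockets at camera-trace hits, falling back to camera rotation.
; Charge fraction feeds projectiles, the weapon material and a looping sound.
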(event Custom|DisableWeaponFire
  (params (Duration :type Float%20%28single-precision%29))
  ;[1 1 1] Disable weapon fire for x seconds
  (Variables|Default|SetIsWeaponFireEnabled false)
  (Utilities|FlowControl|Delay Duration)
  (Variables|Default|SetIsWeaponFireEnabled true))

(event EventBeginPlay
  (Utilities|FlowControl|Sequence
    (:then_0
      ;[1 1 1] Store reference to CombatPowerManager
      (bind _asbp_rbshooter_game_mode (Utilities|Casting|CastToBP_RBShooterGameMode (Game|GetGameMode)))
      (Variables|Default|SetGameMode _asbp_rbshooter_game_mode))
    (:then_1
      ;[1 1 1] Handle Power Tiers and Weapon Attributes
      (|HandlePowerTiers))
    (:then_2
      ;[1 1 1] Disable muzzle flashes
      (Components|Activation|SetActive (Variables|Default|GetMuzzleFlashBlue) false false)
      (Components|Activation|SetActive (Variables|Default|GetMuzzleFlashRed) false false))))

(event EventOnProjectileReleased
  (params (ProjectileType :type EColorTypes%20Enum :default "CT_None") (ChargeFraction :type Float%20%28single-precision%29))
  ;[1 1 1] Projectile Released Event
  (Default|CallOnProjectileReleasedBP ProjectileType ChargeFraction)
  ;;[1 1 1] Set Muzzle Flashes Active
  (Components|Activation|SetActive (Utilities|Select :Index ProjectileType :CT_None 0 :CT_Red (Variables|Default|GetMuzzleFlashRed) :CT_Blue (Variables|Default|GetMuzzleFlashBlue)) true true))

(event EventOnProjectileLoad
  (params (ProjectileType :type EColorTypes%20Enum :default "CT_None"))
  ;[1 1 1] Projectile Load Event
  (|UpdateWeaponMaterial ProjectileType
    (:Exec
      (Default|CallOnProjectileLoadBP ProjectileType)
      (bind _returnvalue (Audio|SpawnSoundAttached "/Game/Sound/Placeholder_Sounds/charge_mockup_Shortend.charge_mockup_Shortend" (Variables|Components|GetWeapon) "None" "0, 0, 0" "0, 0, 0" "KeepRelativeOffset" false 1.0 1.0 0.0 0 0)))))

(event EventOnFireProjectileConfirmed
  (params (ProjectileType :type EColorTypes%20Enum :default "CT_None") (ChargeAmount :type Float%20%28single-precision%29))
  ;[0.9948 1 0.9896] Decide what type of projectile to fire
  (if (Variables|Default|GetbWantsToFirePowerAbility)
    (if (Class|CombatPowerManager|HasBombPoint (Variables|/Game/Gameplay/Blueprints/BP_RBShooterGameMode.BP_RBShooterGameMode_C|GetCombatPowerManager (Variables|Default|GetGameMode)) ProjectileType 1)
      (CallFunction|FirePowerAbility ProjectileType))
    (else
      (switch Utilities|FlowControl|Switch|SwitchonEColorTypes ProjectileType
        (:CT_Red
          ;;[1 0.07061 0] Normal Red
          (CallFunction|SpawnandFireProjectile "/Game/Gameplay/Blueprints/Combat/Projectile/BP_ProjectileRed.BP_ProjectileRed_C" "CT_Red")
          (Audio|PlaySound2D "/Game/Sound/Placeholder_Sounds/S_Fire_Red_Projectile.S_Fire_Red_Projectile" 1.0 (Math|Random|RandomFloatinRange 0.8 1.1) 0.0 0 0))
        (:CT_Blue
          ;;[0 0.6258 1] Normal Blue
          (CallFunction|SpawnandFireProjectile "/Game/Gameplay/Blueprints/Combat/Projectile/BP_ProjectileBlue.BP_ProjectileBlue_C" "CT_Blue")
          (Audio|PlaySound2D "/Game/Sound/Placeholder_Sounds/S_FireProjectileBlue2.S_FireProjectileBlue2" 1.0 (Math|Random|RandomFloatinRange 1.0 1.2) 0.0 0 0))))))

(event EventTick
  (params (DeltaSeconds :type Float%20%28single-precision%29))
  (bind _charge_mockup_shortend_endloop_cue (Variables|Default|Getcharge_mockup_Shortend_EndLoop_Cue))
  ;[1 1 1] Update Charge Fraction on material
  (if (Variables|Default|GetbIsChargingWeapon)
    (Utilities|FlowControl|Sequence
      (:then_0
        (Rendering|Material|SetScalarParameterValueonMaterials (Variables|Components|GetWeapon) "ChargeFraction" (Class|Weapon|GetChargeFraction)))
      (:then_1
        (if (>= (Class|Weapon|GetChargeFraction) 0.9)
          (if (not (Audio|Components|Audio|IsPlaying _charge_mockup_shortend_endloop_cue))
            (Audio|Components|Audio|Play _charge_mockup_shortend_endloop_cue 0.0)))))
    (else
      (Audio|Components|Audio|Stop _charge_mockup_shortend_endloop_cue))))

(event Input|ActionEvents|InputActionFireBlueProjectile
  (params (Key :type Key%20Structure :default "None"))
  ;[1 1 1] Fire Projectile Input
  ;;[0 0.4174 1] Load/Release Blue Projectile
  (:Pressed
    (CallFunction|AttempttoLoadProjectile "CT_Blue"))
  (:Released
    (Class|Weapon|ReleaseProjectile "CT_Blue")
    (if (not (Audio|Components|Audio|IsPlaying (Variables|Default|Getcharge_mockup_Shortend_EndLoop_Cue)))
      (Components|DestroyComponent (stale EventOnProjectileLoad _returnvalue)))))

(event Input|ActionEvents|InputActionFireRedProjectile
  (params (Key :type Key%20Structure :default "None"))
  ;[1 1 1] Fire Projectile Input
  ;;[1 0.05385 0] Load/Release Red Projectile
  (:Pressed
    (CallFunction|AttempttoLoadProjectile "CT_Red"))
  (:Released
    (Class|Weapon|ReleaseProjectile "CT_Red")
    (if (not (Audio|Components|Audio|IsPlaying (Variables|Default|Getcharge_mockup_Shortend_EndLoop_Cue)))
      (Components|DestroyComponent (stale EventOnProjectileLoad _returnvalue)))))

(event Input|ActionEvents|InputActionWeaponPowerModifier
  (params (Key :type Key%20Structure :default "None"))
  ;[1 1 1] Fire Projectile Input
  ;;[1 1 1] Weapon Power Hold Modifier
  (:Pressed
    (if (not (Variables|Default|GetbIsChargingWeapon))
      (Variables|Default|SetbWantsToFirePowerAbility true)))
  (:Released
    (Variables|Default|SetbWantsToFirePowerAbility false)))

(fn ConstructionScript)

(fn SpawnandFireProjectile
  (params (Class :type Actor%20Object%20Reference) (Color :type EColorTypes%20Enum :default "CT_None"))
  (bind _returnvalue (Game|GetPlayerCameraManager 0))
  (bind _weapon (Variables|Components|GetWeapon))
  (bind _returnvalue_2 (Transformation|GetSocketLocation _weapon "TopBarrelSocket"))
  (bind _returnvalue_3 (Camera|GetCameraLocation _returnvalue))
  (LocalVariables|SetMuzzleLocation (Utilities|Select :Index Color :CT_None _returnvalue_2 :CT_Red _returnvalue_2 :CT_Blue (Transformation|GetSocketLocation _weapon "BottomBarrelSocket")))
  (LocalVariables|SetLineStart _returnvalue_3)
  (LocalVariables|SetLineEnd (+ _returnvalue_3 (* (Transformation|GetActorForwardVector _returnvalue) (Variables|Default|GetLineTraceMaxDistance))))
  ;[1 1 1] Check if anything is between muzzle and line start, if true don't use line trace to aim
  (bind _returnvalue_4 (Collision|LineTraceByChannel (LocalVariables|GetLineStart) (LocalVariables|GetMuzzleLocation) "TraceTypeQuery4" false (Utilities|Array|MakeArray (Actor|GetParentActor)) "None" true "(R=1.000000,G=0.000000,B=0.998311,A=1.000000)"))
  (if _returnvalue_4
    ;[1 1 1] Make projectile spawn transform
    (LocalVariables|SetSpawnRotation (Camera|GetCameraRotation (Game|GetPlayerCameraManager 0)) :!label _label) ; Both line traces failed, fire anyway (less accurate and probably won't hit anything)
    (else
      ;[1 1 1] First Line Trace- check against Aimable (enemies mostly)
      (bind (_outhit _returnvalue_5) (Collision|LineTraceByChannel (LocalVariables|GetLineStart) (LocalVariables|GetLineEnd) "TraceTypeQuery3" false 0 "None" true "(R=1.000000,G=0.000000,B=0.000000,A=1.000000)" "(R=0.000000,G=0.037146,B=1.000000,A=1.000000)"))
      (if _returnvalue_5
        (LocalVariables|SetLineHit (.Location (Collision|BreakHitResult _outhit)))
        (LocalVariables|SetSpawnRotation (Math|Rotator|FindLookatRotation (LocalVariables|GetMuzzleLocation) (LocalVariables|GetLineHit)))
        (else
          (goto _label)))))
  ;[1 1 1] Spawn and fire the projectile
  (bind _returnvalue_6 (Game|SpawnActorfromClass Class (Math|Transform|MakeTransform (LocalVariables|GetMuzzleLocation) (LocalVariables|GetSpawnRotation)) "Undefined" 0 0))
  (bind _asbp_projectile_base (Utilities|Casting|CastToBP_ProjectileBase _returnvalue_6))
  (bind _output_get (LocalVariables|SetSpawnedProjectile _asbp_projectile_base))
  (Variables|/Script/RBShooter.ProjectileBase|SetChargeFraction _output_get (Class|Weapon|GetChargeFraction))
  (bind _asbp_player_character (Utilities|Casting|CastToBP_PlayerCharacter (Game|GetPlayerCharacter 0)))
  (Class|ProjectileBase|Fire (LocalVariables|GetSpawnedProjectile) _asbp_player_character self)
  (CallFunction|OnProjectileFired (LocalVariables|GetSpawnedProjectile)))

(fn ChargeProjectile
  (params (ProjectileBase :type BP%20Projectile%20Base%20Object%20Reference))
  (Variables|/Script/RBShooter.ProjectileBase|SetBaseDamage ProjectileBase 0.0))

(fn OnProjectileFired
  (params (Projectile :type BP%20Projectile%20Base%20Object%20Reference))
  (if (>= 0.0 1.0)
    (CallFunction|ChargeProjectile Projectile))
  (Camera|PlayWorldCameraShake "/Game/Characters/Player/Blueprints/BP_FireProjectileCameraShake.BP_FireProjectileCameraShake_C" (Transformation|GetWorldLocation (Variables|Components|GetWeapon)) 0.0 5e+02))

(fn UpdatePowerTier
  (params (BombPointColor :type EColorTypes%20Enum :default "CT_None") (BombPointValue :type Integer))
  (switch int BombPointValue
    (:0
      (Class|Weapon|SetPowerTier BombPointColor "PTT_TierNone"))
    (:1
      (Class|Weapon|SetPowerTier BombPointColor "PTT_Tier1"))
    (:2
      (Class|Weapon|SetPowerTier BombPointColor "PTT_Tier2"))
    (:3
      (Class|Weapon|SetPowerTier BombPointColor "PTT_Tier3"))))

(fn FirePowerAbility
  (params (ColorType :type EColorTypes%20Enum :default "CT_None"))
  (Utilities|FlowControl|Sequence
    (:then_0
      (switch Utilities|FlowControl|Switch|SwitchonEPowerTiesTypes (Class|Weapon|GetPowerTierfromColor ColorType)
        (:PTT_Tier1
          ;[0.5477 0.7102 1] Tier 1 - Magnet Projectile
          (switch Utilities|FlowControl|Switch|SwitchonEColorTypes ColorType
            (:CT_None
              (CallFunction|SpawnandFireProjectile "/Game/Gameplay/Blueprints/Combat/Projectile/BP_MagnetProjectileRed.BP_MagnetProjectileRed_C" "CT_Red" :!label _label))
            (:CT_Red
              (goto _label))
            (:CT_Blue
              (CallFunction|SpawnandFireProjectile "/Game/Gameplay/Blueprints/Combat/Projectile/BP_MagnetProjectileBlue.BP_MagnetProjectileBlue_C" "CT_Blue"))))
        (:PTT_Tier2
          ;[0.9816 1 0.4455] Tier 2 - Magnet Grenade
          (CallFunction|SpawnGrenadePower ColorType))
        (:PTT_Tier3
          ;[1 0.519 0.2648] Tier 3 - Zap Dome
          (CallFunction|SpawnZapDomePower ColorType))))
    (:then_1
      ;[1 1 1] Remove all bomb points of color type
      (Class|CombatPowerManager|RemoveBombPoint (Variables|/Game/Gameplay/Blueprints/BP_RBShooterGameMode.BP_RBShooterGameMode_C|GetCombatPowerManager (Variables|Default|GetGameMode)) ColorType -1))
    (:then_2
      ;[1 1 1] Callback
      (CallFunction|OnPowerAbilityFired ColorType (Class|Weapon|GetPowerTierfromColor ColorType)))))

(fn SpawnGrenadePower
  (params (ColorType :type EColorTypes%20Enum :default "CT_None"))
  (bind _currentchargeamount (Variables|Default|GetCurrentChargeAmount))
  (bind _grenadethrowforce (Variables|Default|GetGrenadeThrowForce))
  (Game|SpawnActorfromClass "/Game/Gameplay/Blueprints/Combat/SpecialMechanics/Grenade/BP_Grenade.BP_Grenade_C" (Transformation|GetActorTransform) "Undefined" 0 ColorType (select (>= _currentchargeamount 1.0) (+ (* _currentchargeamount _grenadethrowforce) 5e+02) (+ _grenadethrowforce 5e+02)) (Transformation|GetActorForwardVector (Game|GetPlayerCameraManager 0)) 0))

(fn UpdateProjectileMultiplier
  (params (Color%20Type :type EColorTypes%20Enum :default "CT_None") (Number%20Of%20Bomb%20Points :type Integer))
  (Class|GameUtility|SetValue (Variables|Default|GetDamageBonus) (* (Math|Conversions|ToFloat(Integer) Number%20Of%20Bomb%20Points) 0.25) Color%20Type)
  (Class|GameUtility|SetValue (Variables|Default|GetProjectileMultiplier) (+ (* (Math|Conversions|ToFloat(Integer) Number%20Of%20Bomb%20Points) 0.3) 1.0) Color%20Type))

(fn IsPowerAbilityChargeable
  (params (PowerType :type EPowerTiesTypes%20Enum :default "PTT_TierNone"))
  (switch Utilities|FlowControl|Switch|SwitchonEPowerTiesTypes PowerType
    (:PTT_TierNone
      (return true))
    (:PTT_Tier1
      (return false))
    (:PTT_Tier2
      (return true))
    (:PTT_Tier3
      (return false))))

(fn AttempttoLoadProjectile
  (params (ProjectileType :type EColorTypes%20Enum :default "CT_None"))
  (if (Variables|Default|GetIsWeaponFireEnabled)
    (if (Variables|Default|GetbWantsToFirePowerAbility)
      (if (CallFunction|IsPowerAbilityChargeable (Class|Weapon|GetPowerTierfromColor ProjectileType))
        ;[1 1 1] Start charging the projectile
        (Class|Weapon|LoadProjectile ProjectileType)
        (else
          ;[1 1 1] Instantly release the projectile
          (Class|Weapon|LoadProjectile ProjectileType)
          (Class|Weapon|ReleaseProjectile ProjectileType)))
      (else
        ;[1 1 1] Normal projectile - start charging it
        (Class|Weapon|LoadProjectile ProjectileType)))))

(fn OnPowerAbilityFired
  (params (ColorType :type EColorTypes%20Enum :default "CT_None") (PowerType :type EPowerTiesTypes%20Enum :default "PTT_TierNone"))
  (CallFunction|DisableWeaponFire (Variables|PowerTier|GetPostPowerAbilityWeaponDisableDuration))
  (Default|CallOnWeaponPowerFired ColorType PowerType))

(fn SpawnZapDomePower
  (params (ColorType :type EColorTypes%20Enum :default "CT_None"))
  (Game|SpawnActorfromClass "/Game/Gameplay/Blueprints/Combat/SpecialMechanics/EnemyZapper/BP_EnemyZapperGrenade.BP_EnemyZapperGrenade_C" (Transformation|GetActorTransform) "Undefined" 0 (Transformation|GetActorForwardVector (Game|GetPlayerCameraManager 0)) 1.5e+03 ColorType (CallFunction|GetPlayerCharacterBP) 0))

(event Custom|OnBombPointChanged
  (params (Color%20Type :type EColorTypes%20Enum :default "CT_None") (Number%20Of%20Bomb%20Points :type Integer))
  (CallFunction|UpdatePowerTier Color%20Type Number%20Of%20Bomb%20Points)
  (CallFunction|UpdateProjectileMultiplier Color%20Type Number%20Of%20Bomb%20Points))