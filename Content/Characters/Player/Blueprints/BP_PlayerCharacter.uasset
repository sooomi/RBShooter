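; First-person player character that sets up the camera, weapon reference and HUD widgets, and shows a death screen when its Health component reports death.
; Incoming damage reduces health and triggers shake, sound, knockback and a one-second immunity flag, while dealt damage is broadcast.
; Optional fall damage measures airtime with a dummy timer.
; A cooldown-gated shout spawns knockback actors with recoil, and a bomb-pulse timeline drives FOV and global time dilation.
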(event Custom|HandleDamageTaken
  (params (DamagedActor :type Actor%20Object%20Reference) (Damage :type Float%20%28single-precision%29) (DamageType :type Damage%20Type%20Object%20Reference) (InstigatedBy :type Controller%20Object%20Reference) (DamageCauser :type Actor%20Object%20Reference))
  ;[1 1 1] Taking Damage
  (Class|HealthComponent|RemoveHealth (Variables|Default|GetHealth) Damage DamageCauser)
  (Camera|PlayWorldCameraShake "/Game/Characters/Player/Blueprints/BP_TakeDamageCameraShake.BP_TakeDamageCameraShake_C" (Transformation|GetWorldLocation (Variables|Default|GetFirstPersonCamera)) 0.0 5e+03)
  (Audio|PlaySound2D "/Game/Sound/Placeholder_Sounds/S_Damage.S_Damage" 1.0 1.0 0.0 0 0)
  ;[1 1 1] Knockback
  (Character|LaunchCharacter (* (Math|Vector|GetUnitDirection(Vector) (Transformation|GetWorldLocation (Variables|/Script/Engine.Actor|GetRootComponent DamageCauser)) (Transformation|GetWorldLocation (Variables|Default|GetCapsuleComponent))) (Variables|Default|GetKnockback%20amount)) false false)
  (Variables|Default|SetIsImmune true)
  (Utilities|FlowControl|Delay 1.0)
  (Variables|Default|SetIsImmune false))

(event Custom|HandleDeath
  (params (InvokeActor :type Actor%20Object%20Reference))
  ;[1 1 1] Handle Death
  (CallFunction|CreatePlayerWidget "/Game/UI/Blueprints/Widget/Gameplay/WBP_DeathScreen.WBP_DeathScreen_C" 0 true))

(event EventBeginPlay
  (Utilities|FlowControl|Sequence
    (:then_0
      ;[1 1 1] Store reference to Weapon actor
      (bind _asbp_weapon (Utilities|Casting|CastToBP_Weapon (Variables|/Script/Engine.ChildActorComponent|GetChildActor (Variables|Default|GetWeaponChildActor))))
      (Variables|Default|SetWeapon _asbp_weapon))
    (:then_1
      ;[1 1 1] Set self (fps camera) as view target on controller
      (Variables|/Script/Engine.CameraComponent|SetbUsePawnControlRotation (Variables|Default|GetFirstPersonCamera) true)
      (Game|Player|SetViewTargetwithBlend (Game|GetPlayerController 0) self 0.0 "VTBlend_Linear" 0.0 false))
    (:then_2
      (|CreateWidgets))
    (:then_3
      ;[1 1 1] Taking Damage
      (EventDispatchers|AssignOnTakeAnyDamage (delegate Custom|HandleDamageTaken)))
    (:then_4
      ;[1 1 1] Handle Death
      (EventDispatchers|AssignOnDeath (Variables|Default|GetHealth) (delegate Custom|HandleDeath)))))

(fn ConstructionScript)

(fn TakeFallDamage
  (params (FallTime :type Float%20%28single-precision%29))
  (if (> FallTime (Variables|FallDamage|GetFallTimeThreshold))
    (LocalVariables|SetDamageToTake (Math|Float|Clamp(Float) (* FallTime (Variables|FallDamage|GetFallDamageMultiplier)) 0.0 (Variables|FallDamage|GetFallDamageMax)))
    (Class|HealthComponent|RemoveHealth (Variables|Default|GetHealth) (LocalVariables|GetDamageToTake) self)
    (Audio|PlaySound2D "/Game/Sound/Placeholder_Sounds/S_Damage.S_Damage" 1.0 1.0 0.0 0 0)
    (Camera|PlayWorldCameraShake "/Game/Characters/Player/Blueprints/BP_TakeDamageCameraShake.BP_TakeDamageCameraShake_C" (Transformation|GetActorLocation) 0.0 5e+02)))

(fn DealDamage
  (params (BaseDamage :type Float%20%28single-precision%29) (DamageTarget :type Actor%20Object%20Reference) (DamageTypeClass :type Damage%20Type%20Class%20Reference))
  (bind _returnvalue (Game|Damage|ApplyDamage DamageTarget BaseDamage 0 self DamageTypeClass))
  (Default|CallOnDamageDealt _returnvalue DamageTarget (LocalVariables|GetDamagetypeClass)))

(event Custom|DummyFallEvent
  ;[1 1 1] Handle Fall Damage (if enabled)
)

(event EventOnWalkingOffLedge
  (params (PreviousFloorImpactNormal :type Vector%20%28by%20ref%29 :default "0, 0, 0") (PreviousFloorContactNormal :type Vector%20%28by%20ref%29 :default "0, 0, 0") (PreviousLocation :type Vector%20%28by%20ref%29 :default "0, 0, 0") (TimeDelta :type Float%20%28single-precision%29))
  ;[1 1 1] Handle Fall Damage (if enabled)
  (if (Variables|FallDamage|GetFallDamageEnabled)
    (bind _returnvalue (Utilities|Time|SetTimerbyEvent (delegate Custom|DummyFallEvent) 3.6e+02))
    (Variables|FallDamage|SetFallDamageTimerHandle _returnvalue)))

(event EventOnLanded
  (params (Hit :type Hit%20Result%20Structure%20%28by%20ref%29))
  ;[1 1 1] Handle Fall Damage (if enabled)
  (if (Variables|FallDamage|GetFallDamageEnabled)
    (FallDamage|TakeFallDamage (Class|KismetSystemLibrary|GetTimerElapsedTimeHandle (Variables|FallDamage|GetFallDamageTimerHandle)))
    (Utilities|Time|ClearandInvalidateTimerbyHandle (Variables|FallDamage|GetFallDamageTimerHandle))))

(event Custom|PlayBombPulse
  (params (Speed :type Float%20%28single-precision%29))
  (Utilities|FlowControl|Sequence
    (:then_0
      (bind (_direction _fov _timedilation) (Timeline|BombPulseTimeline PlayFromStart)
        (:Update
          (Camera|SetFieldOfView (Variables|Default|GetFirstPersonCamera) (+ (* _fov 2e+01) (Variables|/Script/Engine.PlayerCameraManager|GetDefaultFOV (Game|GetPlayerCameraManager 0))))
          (Utilities|Time|SetGlobalTimeDilation _timedilation))))
    (:then_1
      (Components|Timeline|SetPlayRate (Variables|Default|GetBombPulseTimeline) Speed))))

(event Input|ActionEvents|InputActionCreateKnockbackEffect
  (params (Key :type Key%20Structure))
  (bind _firstpersoncamera (Variables|Default|GetFirstPersonCamera))
  (:Pressed
    (if (Variables|Default|GetFosRoDahReady)
      (Game|SpawnActorfromClass "/Game/Gameplay/Blueprints/Combat/Projectile/BP_FusRoDahProjectile.BP_FusRoDahProjectile_C" (Math|Transform|MakeTransform (Transformation|GetWorldLocation _firstpersoncamera) (Transformation|GetSocketRotation _firstpersoncamera "None")) "Undefined" 0 self)
      (Game|SpawnActorfromClass "/Game/Gameplay/Blueprints/Combat/SpecialMechanics/BP_KnockbackVolume.BP_KnockbackVolume_C" (Transformation|GetActorTransform) "Undefined" 0 0)
      (Character|LaunchCharacter (* (Math|Vector|GetForwardVector (Variables|Default|GetFirstPersonCamera)) -5e+02) false false)
      (Variables|Default|SetFosRoDahReady false)
      (Utilities|FlowControl|Delay (Variables|Default|GetFosRoDahCooldown))
      (Variables|Default|SetFosRoDahReady true))))