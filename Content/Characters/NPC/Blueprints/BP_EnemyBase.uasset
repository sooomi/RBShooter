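; Base enemy character that damages the player on hit, either with cooldown attacks or as a suicide bomber that spawns BP_Dragonborn and destroys itself.
; Damage feeds a Health component and briefly stuns surviving enemies by pausing AI logic; death notifies the game mode.
; Projectile and explosion overlaps launch it, and EmpowerEnemy grows health, damage and scale up to a cap.
; Death-state and hit-flash functions are empty; Tick draws debug health and capsule.
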(event Custom|Remove%20Health%20On%20Damage%20Taken
  (params (DamagedActor :type Actor%20Object%20Reference) (Damage :type Float%20%28single-precision%29) (DamageType :type Damage%20Type%20Object%20Reference) (InstigatedBy :type Controller%20Object%20Reference) (DamageCauser :type Actor%20Object%20Reference))
  ;[1 1 1] Handle Damage & Death State
  (Class|HealthComponent|RemoveHealth (Variables|Default|GetHealth) Damage DamageCauser)
  (if (not (Game|IsActorBeingDestroyed))
    (CallFunction|EnemyEmissiveMaterialonHIt)
    (CallFunction|Stun)))

(event Custom|Enemy%20Death%20State
  (params (InvokeActor :type Actor%20Object%20Reference))
  ;[1 1 1] Handle Damage & Death State
  (bind _asbp_rbshooter_game_mode (Utilities|Casting|CastToBP_RBShooterGameMode (Game|GetGameMode)))
  (Default|OnEnemyDied _asbp_rbshooter_game_mode self InvokeActor)
  (CallFunction|HandleDeathState)
  (Actor|DestroyActor)
  (Audio|PlaySound2D "/Game/Sound/Placeholder_Sounds/S_Enemy_Death.S_Enemy_Death" 1.0 1.0 0.0 0 0))

(event EventBeginPlay
  (Utilities|FlowControl|Sequence
    (:then_0
      ;[1 1 1] Handle Damage & Death State
      (EventDispatchers|AssignOnTakeAnyDamage (delegate Custom|Remove%20Health%20On%20Damage%20Taken))
      (EventDispatchers|AssignOnDeath (Variables|Default|GetHealth) (delegate Custom|Enemy%20Death%20State)))))

(event EventTick
  (params (DeltaSeconds :type Float%20%28single-precision%29))
  (bind _health (Variables|Default|GetHealth))
  (bind _capsulecomponent (Variables|Default|GetCapsuleComponent))
  (Utilities|FlowControl|Sequence
    (:then_0
      ;[1 1 1] Render Debug info
      (Rendering|Debug|DrawDebugString (Transformation|GetActorLocation) (Utilities|String|BuildString(Float) (Utilities|String|ToString(Float) (Variables|/Script/RBShooter.HealthComponent|GetCurrentHealth _health)) " / " (Variables|/Script/RBShooter.HealthComponent|GetMaxHealth _health) " HP") 0 "(R=0.000000,G=1.000000,B=0.368307,A=1.000000)")
      (Rendering|Debug|DrawDebugCapsule (Physics|GetCenterOfMass _capsulecomponent "None") (Variables|/Script/Engine.CapsuleComponent|GetCapsuleHalfHeight _capsulecomponent) (Components|Capsule|GetScaledCapsuleRadius _capsulecomponent) (Transformation|GetWorldRotation _capsulecomponent) "(R=1.000000,G=0.847989,B=0.000000,A=1.000000)" 0.0 1.0))
    (:then_1
      (if (Variables|Default|GetIsStunned)
        (Utilities|FlowControl|Delay (Variables|Default|GetStunTime))
        (Class|BrainComponent|RestartLogic (Variables|/Script/AIModule.AIController|GetBrainComponent (AI|GetAIController self)))
        (Variables|Default|SetIsStunned false)))))

(event Collision|EventActorBeginOverlap
  (params (OtherActor :type Actor%20Object%20Reference))
  (if (Utilities|ClassIsChildOf (Utilities|GetClass OtherActor) "/Game/Gameplay/Blueprints/Combat/BP_ProjectileBase.BP_ProjectileBase_C")
    (Character|LaunchCharacter (+ (* (Transformation|GetActorForwardVector (Game|GetPlayerCharacter 0)) 1e+03) "0, 0,100.000000") false false)
    (elif (Utilities|ClassIsChildOf (Utilities|GetClass OtherActor) "/Game/Gameplay/Blueprints/Combat/BP_ExplosionBase.BP_ExplosionBase_C")
      (Character|LaunchCharacter (* (Math|Vector|GetUnitDirection(Vector) (Transformation|GetWorldLocation (Variables|/Script/Engine.Actor|GetRootComponent OtherActor)) (Transformation|GetWorldLocation (Variables|Default|GetCapsuleComponent))) 1e+03) false false))))

(event Collision|EventHit
  (params (MyComp :type Primitive%20Component%20Object%20Reference) (Other :type Actor%20Object%20Reference) (OtherComp :type Primitive%20Component%20Object%20Reference) (bSelfMoved :type Boolean) (HitLocation :type Vector :default "0, 0, 0") (HitNormal :type Vector :default "0, 0, 0") (NormalImpulse :type Vector :default "0, 0, 0") (Hit :type Hit%20Result%20Structure%20%28by%20ref%29))
  (bind _returnvalue (Transformation|GetActorTransform))
  (bind _self self)
  ;[1 1 1] Hitting the player
  (if (Utilities|ClassIsChildOf (Utilities|GetClass Other) "/Game/Characters/Player/Blueprints/BP_PlayerCharacter.BP_PlayerCharacter_C")
    ;;[1 1 1] If suicidebomber or not
    (if (Variables|Default|GetSuicideBomber)
      ;;[1 1 1] Sucidebomber
      (Game|Damage|ApplyDamage Other (Variables|Default|GetBaseDamage) 0 _self)
      (Game|SpawnActorfromClass "/Game/Effects/Particles/BP_Dragonborn.BP_Dragonborn_C" (Math|Transform|MakeTransform (Math|Transform|TransformLocation _returnvalue "0, 0, 0") (Math|Transform|TransformRotation _returnvalue "0, 0, 0")) "Undefined" 0 self)
      (Actor|DestroyActor)
      (else
        ;;[1 1 1] Attacking
        (if (Variables|Default|GetCanAttack)
          (Game|Damage|ApplyDamage Other (Variables|Default|GetBaseDamage) 0 _self)
          (Variables|Default|SetCanAttack false)
          (Utilities|FlowControl|Delay (Variables|Default|GetAttackSpeed))
          (Variables|Default|SetCanAttack true))))))

(fn ConstructionScript)

(fn HandleDeathState)

(fn EnemyEmissiveMaterialonHIt)

(fn EmpowerEnemy
  (params (DamageFromPlayer :type Float%20%28single-precision%29))
  (bind _output_get (Variables|Default|SetCurrentEmpowerment (+ DamageFromPlayer (Variables|Default|GetCurrentEmpowerment))))
  (if (not (> _output_get (Variables|Default|GetMaxEmpowerment)))
    (Class|HealthComponent|AddCurrentandMaxHealth (Variables|Default|GetHealth) DamageFromPlayer DamageFromPlayer 0)
    (Variables|Default|SetBaseDamage (+ (Variables|Default|GetBaseDamage) 1.0))
    (Transformation|SetActorScale3D (+ (Transformation|GetActorScale3D) (Math|Conversions|ToVector(Float) (* DamageFromPlayer 0.2))))))

(fn Stun
  (bind _self self)
  (bind _returnvalue (AI|GetAIController _self))
  (AI|Navigation|StopMovement _returnvalue)
  (AI|Logic|StopLogic (Variables|/Script/AIModule.AIController|GetBrainComponent _returnvalue) "")
  (Variables|Default|SetIsStunned true))