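; BP_EnemyBlueSmall is a small blue enemy NPC that sets a fast walk speed and low max health on BeginPlay, after running its parent's setup.
; Taking damage activates a dissolve effect component with a flare-up, driven by the current health percentage.
; Entering the death state spawns a death particle emitter at the actor's location and applies a blue material to it.
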(event EventBeginPlay
  (|CallParentFunction)
  (Variables|/Script/Engine.CharacterMovementComponent|SetMaxWalkSpeed (Variables|Character|GetCharacterMovement) 1e+03)
  (Class|HealthComponent|SetMaxHealth (Variables|Default|GetHealth) 2.0 0))

(event Collision|EventActorBeginOverlap
  (params (OtherActor :type Actor%20Object%20Reference)))

(event EventTick
  (params (DeltaSeconds :type Float%20%28single-precision%29)))

(event EventPlayDamageEffect
  ;[1 1 1] Emissive Material On Hit
  (Default|ActivateEffect (Variables|Default|GetBP_DissolveEffectComponent) (Class|HealthComponent|GetHealthPercentage (Variables|Default|GetHealth)) true))

(event EventHandleDeathState
  ;[1 1 1] Spawn Death Emitter
  (bind _returnvalue (Effects|SpawnEmitteratLocation "/Game/Characters/NPC/Particles/PS_EnemyDeath.PS_EnemyDeath" (Transformation|GetActorLocation)))
  (Rendering|Material|SetMaterial _returnvalue 0 "/Game/Gameplay/Materials/Particle/MI_ParticleEnemyHitBlue.MI_ParticleEnemyHitBlue"))

(fn ConstructionScript)