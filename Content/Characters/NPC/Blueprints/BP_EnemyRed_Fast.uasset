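; BP_EnemyRed_Fast is the fast red enemy NPC Blueprint, adding visual feedback for hits and death on top of its parent class.
; The death-state event spawns a placeholder red death particle emitter at the actor's location.
; The hit event spikes the mesh's EmissiveIntensity briefly, then settles it to a value based on missing health, so the enemy glows brighter as it takes damage.
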(event Collision|EventActorBeginOverlap
  (params (OtherActor :type Actor%20Object%20Reference)))

(event EventTick
  (params (DeltaSeconds :type Float%20%28single-precision%29)))

(event EventBeginPlay
  (|CallParentFunction))

(event EventHandleDeathState
  ;[1 1 1] Spawn Death Emitter
  (Effects|SpawnEmitteratLocation "/Game/Characters/NPC/Particles/Enemy_Death_Particles_Placeholder/PS_Red_EnemyDeath_Placeholder.PS_Red_EnemyDeath_Placeholder" (Transformation|GetActorLocation)))

(event EventEnemyEmissiveMaterialonHIt
  (bind _health (Variables|Default|GetHealth))
  ;[1 1 1] Emissive Material On Hit
  (Rendering|Material|SetScalarParameterValueonMaterials (Variables|Character|GetMesh) "EmissiveIntensity" 1e+02)
  (Utilities|FlowControl|Delay 0.2)
  (Rendering|Material|SetScalarParameterValueonMaterials (Variables|Character|GetMesh) "EmissiveIntensity" (+ (- (Variables|/Script/RBShooter.HealthComponent|GetMaxHealth _health) (Variables|/Script/RBShooter.HealthComponent|GetCurrentHealth _health)) 0.1)))

(fn ConstructionScript)