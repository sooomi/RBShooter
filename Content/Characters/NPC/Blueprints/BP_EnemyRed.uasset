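; BP_EnemyRed is the red enemy NPC Blueprint, a child class that adds its own death and hit visuals.
; On entering the death state it spawns a placeholder red death particle at its location.
; On hit it passes the Health component's percentage to a dissolve effect component.
; An older emissive-intensity flash on the mesh materials remains in the graph but never runs.
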(event Collision|EventActorBeginOverlap
  (params (OtherActor :type Actor%20Object%20Reference)))

(event EventTick
  (params (DeltaSeconds :type Float%20%28single-precision%29)))

(event EventBeginPlay
  (|CallParentFunction))

(event EventHandleDeathState
  ;[1 1 1] Spawn Death Emitter
  (Effects|SpawnEmitteratLocation "/Game/Characters/NPC/Particles/Enemy_Death_Particles_Placeholder/PS_Red_EnemyDeath_Placeholder.PS_Red_EnemyDeath_Placeholder" (Transformation|GetActorLocation)))

(event EventEnemyEmissiveMaterialonHIt
  ;[1 1 1] Emissive Material On Hit
  (Default|ActivateEffect (Variables|Default|GetBP_DissolveEffectComponent) (Class|HealthComponent|GetHealthPercentage (Variables|Default|GetHealth))))

(fn ConstructionScript)