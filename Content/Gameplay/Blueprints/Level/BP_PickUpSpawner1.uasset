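; Pickup spawner actor that, once activated, spawns a pickup at its own transform after a given delay.
; Activate stores the delay and starts a non-looping timer, presumably bound to PickUpTimerFinished, which calls SpawnPickUps.
; SpawnPickUps always spawns despite collisions, indexing PickUpsActorPool with a random range whose Min (last index) and Max (zero) are reversed.
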(event Custom|PickUpTimerFinished
  (CallFunction|SpawnPickUps))

(event EventBeginPlay)

(event Collision|EventActorBeginOverlap
  (params (OtherActor :type Actor%20Object%20Reference)))

(fn ConstructionScript)

(fn SpawnPickUps
  (bind _pickupsactorpool (Variables|Default|GetPickUpsActorPool))
  (Game|SpawnActorfromClass (Utilities|Array|Get(acopy) _pickupsactorpool (Math|Random|RandomIntegerinRange (- (Utilities|Array|Length _pickupsactorpool) 1) 0)) (Transformation|GetActorTransform) "AlwaysSpawn" 0 0))

(fn Activate
  (params (Delay :type Float%20%28single-precision%29))
  (bind _output_get (Variables|Default|SetPickUpDelay Delay))
  (bind _returnvalue (Utilities|Time|SetTimerbyEvent (EventDispatchers|CreateEvent :!event Custom|PickUpTimerFinished) _output_get))
  (Variables|Default|SetSpawnTimerHandle _returnvalue))