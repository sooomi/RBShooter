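; BP_EnemySpawnNode is a level spawn point that creates a random enemy from its pool with a telegraphed, color-coded entrance.
; ActivateSpawn spawns the enemy and its controller, fires OnSpawnActivated, and returns the enemy.
; That event holds the enemy inactive during a three-second Niagara effect matched to its color type.
; It then removes the effect, activates the enemy, plays a sound and spawns a BP_SpawnLight of matching color.
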(event Custom|OnSpawnActivated
  (params (SpawnedEnemy :type BP%20Enemy%20Base%20Object%20Reference))
  (if (Utilities|IsValid (Variables|Default|GetSpawnEmitter))
    (Components|DestroyComponent (Variables|Default|GetSpawnEmitter)))
  (Default|SetEnemyActive SpawnedEnemy false)
  (bind _returnvalue (Niagara|SpawnSystemAttached (Utilities|Select :Index (Variables|/Script/RBShooter.Enemy|GetEnemyType SpawnedEnemy) :CT_None "/Game/Effects/Particles/Niagara/EnemySpawnMaterialize/NS_EnemySpawnTest1.NS_EnemySpawnTest1" :CT_Red "/Game/Effects/Particles/Niagara/EnemySpawnMaterialize/Placeholder/NS_EnemySpawnTestRed.NS_EnemySpawnTestRed" :CT_Blue "/Game/Effects/Particles/Niagara/EnemySpawnMaterialize/Placeholder/NS_EnemySpawnTestBlue.NS_EnemySpawnTestBlue") (Variables|Default|GetDefaultSceneRoot) "None" (+ (Transformation|GetActorLocation SpawnedEnemy) "0, 0,-50.000000") (Math|Rotator|CombineRotators (Transformation|GetActorRotation SpawnedEnemy) "0,-90.000000, 0") "KeepWorldPosition" false))
  (bind _output_get (Variables|Default|SetSpawnEmitter _returnvalue))
  (Transformation|SetRelativeScale3D _output_get (Transformation|GetActorScale3D))
  (Utilities|FlowControl|Delay 3.0)
  (Components|DestroyComponent (Variables|Default|GetSpawnEmitter))
  (Default|SetEnemyActive SpawnedEnemy true)
  (Audio|PlaySoundatLocation "/Game/Sound/Placeholder_Sounds/S_Spawn.S_Spawn" (Transformation|GetWorldLocation (Variables|Default|GetDefaultSceneRoot)) "0, 0, 0" 1.0 1.0 0.0 0 0 0)
  (bind _returnvalue_2 (Game|SpawnActorfromClass "/Game/Gameplay/Blueprints/Level/BP_SpawnLight.BP_SpawnLight_C" (Transformation|GetActorTransform) "Undefined" 0 0))
  (Variables|/Game/Gameplay/Blueprints/Level/BP_SpawnLight.BP_SpawnLight_C|SetColorType _returnvalue_2 (Variables|/Script/RBShooter.Enemy|GetEnemyType SpawnedEnemy)))

(event EventBeginPlay)

(event EventOnSpawnSelected
  (params (TimeUntilFirstSpawn :type Float%20%28single-precision%29)))

(fn ConstructionScript)

(fn ActivateSpawn
  (bind _enemyactorpool (Variables|Default|GetEnemyActorPool))
  (bind _returnvalue (Game|SpawnActorfromClass (Utilities|Array|Get(acopy) _enemyactorpool (Math|Random|RandomIntegerinRange 0 (- (Utilities|Array|Length _enemyactorpool) 1))) (Math|Transform|MakeTransform (Transformation|GetActorLocation) (Transformation|GetActorRotation)) "AlwaysSpawn" 0 0))
  (bind _asbp_enemy_base (Utilities|Casting|CastToBP_EnemyBase _returnvalue))
  (bind _output_get (LocalVariables|SetSpawnedEnemy _asbp_enemy_base))
  (Pawn|SpawnDefaultController _output_get)
  (Variables|/Game/Characters/NPC/Blueprints/BP_EnemyBase.BP_EnemyBase_C|SetHasSpawned (LocalVariables|GetSpawnedEnemy) true)
  (CallFunction|OnSpawnActivated (LocalVariables|GetSpawnedEnemy))
  (return (LocalVariables|GetSpawnedEnemy)))