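; BP_SpawnLight is a short-lived light effect actor in red or blue, likely marking a spawn.
; On BeginPlay a timeline drives the intensity of two point lights from its Brightness track.
; Each update also sets both lights' color from the ColorType selection.
; The actor destroys itself when the timeline finishes.
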(event EventBeginPlay
  (bind _pointlight (Variables|Default|GetPointLight))
  (bind _brightness (Timeline|Timeline_0 Play)
    (:Update
      (Rendering|Components|Light|SetIntensity (Variables|Default|GetPointLight) (* _brightness 5e+02))
      (switch Utilities|FlowControl|Switch|SwitchonEColorTypes (Variables|Default|GetColorType)
        (:CT_Red
          (Rendering|Components|Light|SetLightColor _pointlight "(R=1.000000,G=0.000000,B=0.000000,A=1.000000)" true))
        (:CT_Blue
          (Rendering|Components|Light|SetLightColor _pointlight "(R=0.000000,G=0.223963,B=1.000000,A=1.000000)" true))))
    (:Finished
      (Actor|DestroyActor))))

(event Collision|EventActorBeginOverlap
  (params (OtherActor :type Actor%20Object%20Reference)))

(event EventTick
  (params (DeltaSeconds :type Float%20%28single-precision%29)))

(fn ConstructionScript)