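; BP_Laserwall is a level hazard that kills the player, enemies or both on overlap, depending on two flags.
; Overlap checks the actor's class against BP_PlayerCharacter and BP_EnemyBase, then calls Kill on its Health.
; Tick uses Delays of TimeExisting to alternate the Active state.
; The wall switches off by teleport-free moving 1000 units down and returns to the transform saved at BeginPlay.
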(event EventBeginPlay
  (Variables|Default|SetStarting%20possition (Transformation|GetActorTransform)))

(event Collision|EventActorBeginOverlap
  (params (OtherActor :type Actor%20Object%20Reference))
  (if (or (Variables|Default|GetDoesKillPlayer) (Variables|Default|GetDoesKillEnemy))
    (if (and (Utilities|ClassIsChildOf (Utilities|GetClass OtherActor) "/Game/Characters/Player/Blueprints/BP_PlayerCharacter.BP_PlayerCharacter_C") (Variables|Default|GetDoesKillPlayer))
      (bind _asbp_player_character (Utilities|Casting|CastToBP_PlayerCharacter OtherActor))
      (Class|HealthComponent|Kill (Variables|/Game/Characters/Player/Blueprints/BP_PlayerCharacter.BP_PlayerCharacter_C|GetHealth _asbp_player_character) 0))
    (if (and (Utilities|ClassIsChildOf (Utilities|GetClass OtherActor) "/Game/Characters/NPC/Blueprints/BP_EnemyBase.BP_EnemyBase_C") (Variables|Default|GetDoesKillEnemy))
      (bind _asbp_enemy_base (Utilities|Casting|CastToBP_EnemyBase OtherActor))
      (Class|HealthComponent|Kill (Variables|/Game/Characters/NPC/Blueprints/BP_EnemyBase.BP_EnemyBase_C|GetHealth _asbp_enemy_base) 0))))

(event EventTick
  (params (DeltaSeconds :type Float%20%28single-precision%29))
  (bind _time_existing (Variables|Default|GetTime%20Existing))
  (if (Variables|Default|GetActive)
    (Utilities|FlowControl|Delay _time_existing)
    (Transformation|SetActorLocation (+ (Transformation|GetActorLocation) "0, 0,-1000.000000") false false)
    (Variables|Default|SetActive false)
    (else
      (Utilities|FlowControl|Delay _time_existing)
      (Transformation|SetActorTransform (Variables|Default|GetStarting%20possition))
      (Variables|Default|SetActive true))))

(fn ConstructionScript)