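; BP_PickUpSpawner is a level actor that places a random pickup at its own transform.
; SpawnPickUp destroys overlapping BP_PickUp_Base actors, then always spawns a random class from PickupActorPool, regardless of collision.
; If the spawned actor is a BP_EnemyBase, it also spawns that enemy's default controller, so the pool can supply enemies as well as pickups.
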(fn ConstructionScript)

(fn SpawnPickUp
  (bind _pickupactorpool (Variables|Default|GetPickupActorPool))
  (Actor|DestroyActor (Collision|GetOverlappingActors "/Game/Gameplay/Blueprints/PickUp/BP_Pick-Up_Base.BP_Pick-Up_Base_C" :!class /Script/Engine.Actor))
  (bind _returnvalue (Game|SpawnActorfromClass (Utilities|Array|Get(acopy) _pickupactorpool (Math|Random|RandomIntegerinRange 0 (- (Utilities|Array|Length _pickupactorpool) 1))) (Transformation|GetActorTransform) "AlwaysSpawn" 0 0))
  (bind _asbp_enemy_base (Utilities|Casting|CastToBP_EnemyBase _returnvalue))
  (Pawn|SpawnDefaultController _asbp_enemy_base))