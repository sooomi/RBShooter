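; BP_PhysicsBox is a level physics prop that gets shoved when hit by projectiles or knockback volumes.
; On actor overlap it checks whether the other actor derives from the FusRoDah projectile, base projectile or knockback volume classes.
; A match overrides the cube's linear velocity with a fixed-speed push along the player character's forward vector, regardless of where the hit came from.
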(event EventBeginPlay)

(event Collision|EventActorBeginOverlap
  (params (OtherActor :type Actor%20Object%20Reference))
  (bind _returnvalue (Utilities|GetClass OtherActor))
  (if (Math|Boolean|ORBoolean (Utilities|ClassIsChildOf _returnvalue "/Game/Gameplay/Blueprints/Combat/Projectile/BP_FusRoDahProjectile.BP_FusRoDahProjectile_C") (Utilities|ClassIsChildOf _returnvalue "/Game/Gameplay/Blueprints/Combat/Projectile/BP_ProjectileBase.BP_ProjectileBase_C") (Utilities|ClassIsChildOf _returnvalue "/Game/Gameplay/Blueprints/Combat/SpecialMechanics/BP_KnockbackVolume.BP_KnockbackVolume_C"))
    (Physics|SetPhysicsLinearVelocity (Variables|Default|GetCube) (* (Transformation|GetActorForwardVector (Game|GetPlayerCharacter 0)) 5e+02) false "None")))

(fn ConstructionScript)