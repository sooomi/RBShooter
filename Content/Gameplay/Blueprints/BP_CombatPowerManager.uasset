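; Manages red and blue combat power, turning the player's enemy kills into colour timer increases scaled by enemy max health.
; Gaining a bomb point plays pulse and sound feedback and lengthens that colour's max timer.
; Removing points activates a ScoreManager tier bonus and blocks that colour's kill gains for the tier's effect duration, using retriggerable delays.
; Point and timer changes are relayed through Blueprint event calls.
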(event Custom|OnEnemyDied
  (params (Enemy :type BP%20Enemy%20Base%20Object%20Reference) (Killer :type Actor%20Object%20Reference))
  (bind _enemytype (Variables|/Script/RBShooter.Enemy|GetEnemyType Enemy))
  (if (== Killer (Game|GetPlayerCharacter 0))
    (switch Utilities|FlowControl|Switch|SwitchonEColorTypes _enemytype
      (:CT_Red
        (if (not (Variables|Default|GetHasRecentlyUsedRedPower))
          (Class|CombatPowerManager|IncreaseTimer (Variables|/Script/RBShooter.HealthComponent|GetMaxHealth (Variables|/Game/Characters/NPC/Blueprints/BP_EnemyBase.BP_EnemyBase_C|GetHealth Enemy)) _enemytype :!label _label)))
      (:CT_Blue
        (if (not (Variables|Default|GetHasRecentlyUsedBluePower))
          (goto _label))))))

(event EventBeginPlay
  (bind _asbp_rbshooter_game_mode (Utilities|Casting|CastToBP_RBShooterGameMode (Game|GetGameMode)))
  (EventDispatchers|BindEventtoOnEnemyDiedBP _asbp_rbshooter_game_mode (EventDispatchers|CreateEvent :!event Custom|OnEnemyDied)))

(event EventOnBombPointRemoved
  (params (ColorType :type EColorTypes%20Enum :default "CT_None") (NumPointsNow :type Integer) (NumPointsBefore :type Integer))
  (CallFunction|HandleBombPointRemoval ColorType NumPointsBefore)
  (Default|CallOnBombPointRemovedBP ColorType NumPointsNow NumPointsBefore)
  (Default|CallOnBombPointChangedBP ColorType NumPointsNow NumPointsBefore))

(event EventOnBombPointAdded
  (params (ColorType :type EColorTypes%20Enum :default "CT_None") (NumPointsNow :type Integer) (NumPointsBefore :type Integer))
  (bind _maxtimeblue (Variables|Default|GetMaxTimeBlue))
  (bind _maxtimered (Variables|Default|GetMaxTimeRed))
  (bind _returnvalue (Utilities|Select :Index ColorType :CT_None 0.0 :CT_Red _maxtimered :CT_Blue _maxtimeblue))
  (Default|CallOnBombPointAddedBP ColorType NumPointsNow NumPointsBefore)
  (Default|CallOnBombPointChangedBP ColorType NumPointsNow NumPointsBefore)
  (Default|PlayBombPulse (CallFunction|GetPlayerCharacterBP) 1.5)
  (Audio|SpawnSound2D "/Game/Sound/Placeholder_Sounds/S_Gunpoint.S_Gunpoint" 1.0 1.0 0.0 0)
  (Audio|PlaySound2D "/Game/Sound/Placeholder_Sounds/S_SlowMo.S_SlowMo" 1.0 1.0 0.0 0 0)
  (|SetBy-RefVar _returnvalue (+ _returnvalue (Variables|Default|GetTimerIncrease))))

(event EventOnTimerUpdated
  (params (ColorType :type EColorTypes%20Enum :default "CT_None"))
  (Default|CallOnTimerUpdatedBP ColorType))

(event EventOnTimerStarted
  (params (ColorType :type EColorTypes%20Enum :default "CT_None"))
  (Default|CallOnTimerStartedBP ColorType))

(event EventOnTimerEnded
  (params (ColorType :type EColorTypes%20Enum :default "CT_None"))
  (Default|CallOnTimerEndedBP ColorType))

(fn ConstructionScript)

(fn GetPowerTierEffectDuration
  (params (PowerTtype :type EPowerTiesTypes%20Enum :default "PTT_TierNone"))
  (return (Utilities|Select :Index PowerTtype :PTT_TierNone 0.0 :PTT_Tier1 8.0 :PTT_Tier2 6.0 :PTT_Tier3 15.0)))

(event Custom|HandleBombPointRemoval
  (params (ColorType :type EColorTypes%20Enum :default "CT_None") (NumberOfBombPoints :type Integer))
  (bind _returnvalue (Utilities|Select :Index NumberOfBombPoints :Option%200 "PTT_TierNone" :Option%201 "PTT_Tier1" :Option%202 "PTT_Tier2" :Option%203 "PTT_Tier3"))
  (bind _returnvalue_2 (CallFunction|GetPowerTierEffectDuration _returnvalue))
  (Utilities|FlowControl|Sequence
    (:then_0
      (Class|ScoreManager|ActivateTierBonus (Variables|/Script/RBShooter.RBShooterGameModeBase|GetScoreManager (CallFunction|GetGameModeBP)) ColorType _returnvalue 0.3 (CallFunction|GetPowerTierEffectDuration _returnvalue)))
    (:then_1
      (switch Utilities|FlowControl|Switch|SwitchonEColorTypes ColorType
        (:CT_Red
          (Variables|Default|SetHasRecentlyUsedRedPower true)
          (Utilities|FlowControl|RetriggerableDelay _returnvalue_2)
          (Variables|Default|SetHasRecentlyUsedRedPower false))
        (:CT_Blue
          (Variables|Default|SetHasRecentlyUsedBluePower true)
          (Utilities|FlowControl|RetriggerableDelay _returnvalue_2)
          (Variables|Default|SetHasRecentlyUsedBluePower false))))))