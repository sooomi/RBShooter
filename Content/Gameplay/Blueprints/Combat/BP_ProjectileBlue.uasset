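; Blue variant of a combat projectile that supplies color-specific impact effects.
; BeginPlay defers to the parent class, and the matching and mismatching hit events each spawn their own blue particle emitter at the projectile's location, then destroy the actor.
; The logic that decides whether a hit matches is not in this Blueprint.
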(event EventBeginPlay
  (|CallParentFunction))

(event Collision|EventActorBeginOverlap
  (params (OtherActor :type Actor%20Object%20Reference)))

(event EventTick
  (params (DeltaSeconds :type Float%20%28single-precision%29)))

(event EventHandleMismatchingHit
  ;[1 1 1] Spawn Emitter on Mismatching hit
  (Effects|SpawnEmitteratLocation "/Game/Gameplay/Particles/Projectile_Hit_Particles/PS_Blue_Mismatching_Hit_Projectile.PS_Blue_Mismatching_Hit_Projectile" (Transformation|GetActorLocation self))
  (Actor|DestroyActor))

(event EventHandleMatchingHit
  ;[1 1 1] Spawn Emitter on Mismatching hit
  (Effects|SpawnEmitteratLocation "/Game/Gameplay/Particles/Projectile_Hit_Particles/PS_Blue_Matching_Hit_Projectile.PS_Blue_Matching_Hit_Projectile" (Transformation|GetActorLocation self))
  (Actor|DestroyActor))

(fn ConstructionScript)