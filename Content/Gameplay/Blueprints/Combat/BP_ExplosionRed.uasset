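; BP_ExplosionRed is a short-lived explosion actor that damages color-matched enemies it overlaps.
; It destroys itself half a second after BeginPlay.
; On overlap with a BP_EnemyBase child, it compares its Color to the enemy's EnemyType and applies damage only on a match, naming the player character as damage causer.
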(event EventBeginPlay
  (Utilities|FlowControl|Delay 0.5)
  (Actor|DestroyActor))

(event Collision|EventActorBeginOverlap
  (params (OtherActor :type Actor%20Object%20Reference))
  (if (Utilities|ClassIsChildOf (Utilities|GetClass OtherActor) "/Game/Characters/NPC/Blueprints/BP_EnemyBase.BP_EnemyBase_C")
    (bind _asbp_enemy_base (Utilities|Casting|CastToBP_EnemyBase OtherActor))
    (if (Utilities|Enum|Equal(Enum) (Variables|Default|GetColor) (Variables|/Script/RBShooter.Enemy|GetEnemyType _asbp_enemy_base))
      (Game|Damage|ApplyDamage OtherActor 1.0 0 (Game|GetPlayerCharacter 0)))))

(event EventTick
  (params (DeltaSeconds :type Float%20%28single-precision%29)))

(fn ConstructionScript)