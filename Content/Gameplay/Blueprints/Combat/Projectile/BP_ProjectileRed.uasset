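; Red variant of a combat projectile Blueprint, extending a parent that provides the base BeginPlay and hit handling events.
; On BeginPlay, a timeline spins the mesh around its roll axis while keeping pitch and yaw.
; Matching hits spawn the enemy-hit particle at the projectile's location, tinted red through material and color parameter.
; Mismatching hits spawn a dedicated red mismatch particle instead.
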(event EventBeginPlay
  (bind _mesh (Variables|Default|GetMesh))
  (bind _returnvalue (Transformation|GetWorldRotation _mesh))
  (bind (_roll _pitch _yaw) (Math|Rotator|BreakRotator _returnvalue))
  (|CallParentFunction)
  (bind _rotation (Timeline|MeshAnimation Play)
    (:Update
      (Transformation|SetWorldRotation (Variables|Default|GetMesh) (Math|Rotator|MakeRotator (* (* _rotation 1e+01) 3.6e+02) _pitch _yaw) false false))))

(event Collision|EventActorBeginOverlap
  (params (OtherActor :type Actor%20Object%20Reference)))

(event EventTick
  (params (DeltaSeconds :type Float%20%28single-precision%29)))

(event EventHandleMismatchingHit
  (params (Enemy :type Actor%20Object%20Reference))
  ;[1 1 1] Spawn Emitter On Mismatching Hit
  (Effects|SpawnEmitteratLocation "/Game/Gameplay/Particles/ProjectileHit/PH/PS_Red_Mismatching_Hit_Projectile.PS_Red_Mismatching_Hit_Projectile" (Transformation|GetActorLocation self)))

(event EventHandleMatchingHit
  (params (Enemy :type Actor%20Object%20Reference))
  ;[1 1 1] Spawn Emitter On Matching Hit
  (bind _returnvalue (Effects|SpawnEmitteratLocation "/Game/Gameplay/Particles/ProjectileHit/PS_ProjectileEnemyHit.PS_ProjectileEnemyHit" (Transformation|GetActorLocation)))
  (Rendering|Material|SetMaterial _returnvalue 0 "/Game/Gameplay/Materials/Particle/MI_ParticleEnemyHitRed.MI_ParticleEnemyHitRed")
  (Effects|Components|ParticleSystem|SetColorParameter _returnvalue "Color" "(R=1.000000,G=0.000000,B=0.012817,A=1.000000)"))

(fn ConstructionScript)