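; Fus Ro Dah shout projectile that briefly stuns overlapped BP_EnemyBase enemies and launches them along its forward vector with a fixed upward lift.
; Tick steadily reduces knockback strength and shrinks the actor, so later hits push less.
; BeginPlay removes a secondary sphere and sets a Niagara weight, then after short delays drops the main sphere, deactivates the effect and destroys the actor.
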(event EventBeginPlay
  (Components|DestroyComponent (Variables|Default|GetSphere1))
  (Class|NiagaraComponent|SetNiagaraVariableVec3 (Variables|Default|GetNiagara) "User.Weight" "0, 0,-300.000000")
  (Utilities|FlowControl|Delay 0.75)
  (Components|DestroyComponent (Variables|Default|GetSphere))
  (Components|Activation|Deactivate (Variables|Default|GetNiagara))
  (Utilities|FlowControl|Delay 1.0)
  (Actor|DestroyActor))

(event Collision|EventActorBeginOverlap
  (params (OtherActor :type Actor%20Object%20Reference))
  (if (Utilities|ClassIsChildOf (Utilities|GetClass OtherActor) "/Game/Characters/NPC/Blueprints/BP_EnemyBase.BP_EnemyBase_C")
    (bind _asbp_enemy_base (Utilities|Casting|CastToBP_EnemyBase OtherActor))
    (Default|Stun _asbp_enemy_base 0.5)
    (Character|LaunchCharacter _asbp_enemy_base (+ (* (Transformation|GetActorForwardVector) (Variables|Default|GetKnockback%20amount)) "0, 0,250.000000") true true)))

(event EventTick
  (params (DeltaSeconds :type Float%20%28single-precision%29))
  (Variables|Default|SetKnockback%20Amount (- (Variables|Default|GetKnockback%20Amount) (* DeltaSeconds (Variables|Default|GetReduction%20multiplier))))
  (Transformation|SetActorScale3D (- (Transformation|GetActorScale3D) DeltaSeconds)))

(fn ConstructionScript)