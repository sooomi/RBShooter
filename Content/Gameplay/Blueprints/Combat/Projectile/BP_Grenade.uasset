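; BP_Grenade is a projectile that detonates after a short fuse, or immediately when it hits an enemy derived from BP_EnemyBase.
; Both triggers share one detonation path at the Sphere's transform, which spawns a BP_ExplosionBase set to ignore color plus a brief BP_EnemyMagnetEffect with no enemy type.
; The grenade then destroys itself.
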(event EventBeginPlay
  (bind _self self)
  (bind _sphere (Variables|Default|GetSphere _self))
  (bind _returnvalue (Transformation|GetWorldTransform _sphere))
  (Utilities|FlowControl|Delay 2.5)
  (bind _returnvalue_2 (Game|SpawnActorfromClass "/Game/Gameplay/Blueprints/Combat/SpecialMechanics/BP_ExplosionBase.BP_ExplosionBase_C" _returnvalue "Undefined" 0 0))
  (Variables|/Game/Gameplay/Blueprints/Combat/SpecialMechanics/BP_ExplosionBase.BP_ExplosionBase_C|SetIgnoreColor _returnvalue_2 true)
  (Game|SpawnActorfromClass "/Game/Gameplay/Blueprints/Combat/SpecialMechanics/BP_EnemyMagnetEffect.BP_EnemyMagnetEffect_C" _returnvalue "Undefined" 0 1.0 "CT_None" 0)
  (Actor|DestroyActor))

(event EventTick
  (params (DeltaSeconds :type Float%20%28single-precision%29)))

(event Collision|EventHit
  (params (MyComp :type Primitive%20Component%20Object%20Reference) (Other :type Actor%20Object%20Reference) (OtherComp :type Primitive%20Component%20Object%20Reference) (bSelfMoved :type Boolean) (HitLocation :type Vector :default "0, 0, 0") (HitNormal :type Vector :default "0, 0, 0") (NormalImpulse :type Vector :default "0, 0, 0") (Hit :type Hit%20Result%20Structure%20%28by%20ref%29))
  (bind _self self)
  (bind _sphere (Variables|Default|GetSphere _self))
  (bind _returnvalue (Transformation|GetWorldTransform _sphere))
  (if (Utilities|ClassIsChildOf (Utilities|GetClass Other) "/Game/Characters/NPC/Blueprints/BP_EnemyBase.BP_EnemyBase_C")
    (bind _returnvalue_2 (Game|SpawnActorfromClass "/Game/Gameplay/Blueprints/Combat/SpecialMechanics/BP_ExplosionBase.BP_ExplosionBase_C" _returnvalue "Undefined" 0 0))
    (Variables|/Game/Gameplay/Blueprints/Combat/SpecialMechanics/BP_ExplosionBase.BP_ExplosionBase_C|SetIgnoreColor _returnvalue_2 true)
    (Game|SpawnActorfromClass "/Game/Gameplay/Blueprints/Combat/SpecialMechanics/BP_EnemyMagnetEffect.BP_EnemyMagnetEffect_C" _returnvalue "Undefined" 0 1.0 "CT_None" 0)
    (Actor|DestroyActor)))

(fn ConstructionScript)