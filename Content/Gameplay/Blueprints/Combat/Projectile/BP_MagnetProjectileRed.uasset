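; Red magnet projectile that places a red enemy magnet effect where it hits.
; When its sphere component begins overlapping another actor, it spawns BP_EnemyMagnetEffect at its own transform with the Red enemy type, then destroys itself after a short delay.
; The overlap does not filter by actor type beyond excluding itself, and the OnProjectileHitEnemy event is left empty.
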(event OnComponentBeginOverlap(EditorSphereComponent)
  (params (OverlappedComponent :type Primitive%20Component%20Object%20Reference) (OtherActor :type Actor%20Object%20Reference) (OtherComp :type Primitive%20Component%20Object%20Reference) (OtherBodyIndex :type Integer) (bFromSweep :type Boolean) (SweepResult :type Hit%20Result%20Structure%20%28by%20ref%29))
  (if (!= OtherActor self)
    (Game|SpawnActorfromClass "/Game/Gameplay/Blueprints/Combat/SpecialMechanics/BP_EnemyMagnetEffect.BP_EnemyMagnetEffect_C" (Transformation|GetActorTransform) "Undefined" 0 8.0 "CT_Red" 0)
    (Utilities|FlowControl|Delay 0.1)
    (Actor|DestroyActor)))

(event EventBeginPlay
  (|CallParentFunction) ; This node is disabled and will not be called.\nDrag off pins to build functionality.
)

(event EventOnProjectileHitEnemy
  (params (Enemy :type Enemy%20Object%20Reference) (bColorMatch :type Boolean) (Damage :type Float%20%28single-precision%29)))

(fn ConstructionScript
  (|CallParentFunction))