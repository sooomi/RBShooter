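; BP_ProjectileBlue is the blue color variant of a combat projectile, extending parent behavior with its own visuals and explosion.
; A timeline started on BeginPlay spins the mesh around its roll axis.
; Matching and mismatching hit events spawn different particle effects at the projectile, the matching one recolored with a blue material.
; SpawnExplosion creates a blue explosion actor, using ChargeAmount for both its scale and damage.
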(event EventBeginPlay
  (bind _mesh (Variables|Default|GetMesh))
  (bind _returnvalue (Transformation|GetWorldRotation _mesh))
  (bind (_roll _pitch _yaw) (Math|Rotator|BreakRotator _returnvalue))
  (|CallParentFunction)
  (bind _rotation (Timeline|MeshAnimation Play)
    (:Update
      (Transformation|SetWorldRotation (Variables|Default|GetMesh) (Math|Rotator|MakeRotator (* (* _rotation 1e+01) 3.6e+02) _pitch _yaw) false false))))

(event Collision|EventActorBeginOverlap
  (params (OtherActor :type Actor%20Object%20Reference)))

(event EventTick
  (params (DeltaSeconds :type Float%20%28single-precision%29)))

(event EventSpawnExplosion
  (bind _self self)
  (bind _returnvalue (Game|SpawnActorfromClass "/Game/Gameplay/Blueprints/Combat/SpecialMechanics/Explosion/BP_ExplosionBlue1.BP_ExplosionBlue1_C" (Math|Transform|MakeTransform (Transformation|GetActorLocation _self) (Transformation|GetActorRotation _self) (Math|Conversions|ToVector(Float) (Variables|Default|GetChargeAmount))) "Undefined" 0 "CT_Blue" 0))
  (Variables|/Game/Gameplay/Blueprints/Combat/SpecialMechanics/Explosion/BP_ExplosionBase.BP_ExplosionBase_C|SetExplosionDamage _returnvalue (Variables|Default|GetChargeAmount)))

(event EventHandleMismatchingHit
  (params (Enemy :type Actor%20Object%20Reference))
  ;[1 1 1] Spawn Emitter on Mismatching hit
  (Effects|SpawnEmitteratLocation "/Game/Gameplay/Particles/ProjectileHit/PH/PS_Blue_Mismatching_Hit_Projectile.PS_Blue_Mismatching_Hit_Projectile" (Transformation|GetActorLocation self)))

(event EventHandleMatchingHit
  (params (Enemy :type Actor%20Object%20Reference))
  ;[1 1 1] Spawn Emitter on Matching hit
  (bind _returnvalue (Effects|SpawnEmitteratLocation "/Game/Gameplay/Particles/ProjectileHit/PS_ProjectileEnemyHit.PS_ProjectileEnemyHit" (Transformation|GetActorLocation)))
  (Rendering|Material|SetMaterial _returnvalue 0 "/Game/Gameplay/Materials/Particle/MI_ParticleEnemyHitBlue.MI_ParticleEnemyHitBlue"))

(fn ConstructionScript)