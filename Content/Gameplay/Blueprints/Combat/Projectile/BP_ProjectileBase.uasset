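; Base colour-typed projectile that damages enemies of matching colour and empowers mismatched ones.
; On overlap with a target component, it tests head, chest and leg colliders to scale damage, slows on leg hits, and notifies the enemy.
; Empty matching and mismatching handlers act as hooks for child classes.
; Sufficiently charged shots spawn an explosion on enemy or blocking hits, the latter also playing colour-specific impact effects and sound.
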(event OnComponentBeginOverlap(EditorSphereComponent)
  (params (OverlappedComponent :type Primitive%20Component%20Object%20Reference) (OtherActor :type Actor%20Object%20Reference) (OtherComp :type Primitive%20Component%20Object%20Reference) (OtherBodyIndex :type Integer) (bFromSweep :type Boolean) (SweepResult :type Hit%20Result%20Structure%20%28by%20ref%29))
  ;[1 1 1] Event Begin Overlap - Check enemy hit locations
  (if (Components|ComponentHasTag OtherComp "ProjectileTarget")
    (bind _asbp_enemy_base (Utilities|Casting|CastToBP_EnemyBase OtherActor))
    (if (Utilities|IsValid _asbp_enemy_base)
      (CallFunction|HandleEnemyHit _asbp_enemy_base (Utilities|Enum|Equal(Enum) (Variables|/Script/RBShooter.Enemy|GetEnemyType _asbp_enemy_base) (Variables|Default|GetProjectileType)) (Class|ProjectileBase|GetDamage))
      (if (>= (Variables|Default|GetChargeFraction) 0.33)
        (CallFunction|SpawnExplosion))
      (Rendering|SetActorHiddenInGame false)
      (Actor|Tick|SetActorTickEnabled false)
      (Collision|SetActorEnableCollision false)
      (Utilities|FlowControl|Delay 0.0)
      (Actor|DestroyActor))))

(event Custom|OnProjectileHitEnemy_1
  (params (Enemy :type Enemy%20Object%20Reference) (bColorMatch :type Boolean) (Damage :type Float%20%28single-precision%29))
  ;[0 0 0] Ignore this - collision is done in blueprint only
)

(event EventBeginPlay)

(event EventOnProjectileFired)

(event Collision|EventHit
  (params (MyComp :type Primitive%20Component%20Object%20Reference) (Other :type Actor%20Object%20Reference) (OtherComp :type Primitive%20Component%20Object%20Reference) (bSelfMoved :type Boolean) (HitLocation :type Vector :default "0, 0, 0") (HitNormal :type Vector :default "0, 0, 0") (NormalImpulse :type Vector :default "0, 0, 0") (Hit :type Hit%20Result%20Structure%20%28by%20ref%29))
  ;[1 1 1] Event Hit  - Spawn VFX and Destroy self
  (Effects|SpawnEmitteratLocation (Utilities|Select :Index (Variables|Default|GetProjectileType) :CT_None "/Game/Gameplay/Particles/ProjectileHit/PH/PS_Red_Mismatching_Hit_Projectile.PS_Red_Mismatching_Hit_Projectile" :CT_Red "/Game/Gameplay/Particles/ProjectileHit/PH/PS_Red_Mismatching_Hit_Projectile.PS_Red_Mismatching_Hit_Projectile" :CT_Blue "/Game/Gameplay/Particles/ProjectileHit/PH/PS_Blue_Mismatching_Hit_Projectile.PS_Blue_Mismatching_Hit_Projectile") (Transformation|GetActorLocation))
  (if (>= (Variables|Default|GetChargeFraction) 0.33)
    (CallFunction|SpawnExplosion))
  (Actor|DestroyActor)
  (Audio|PlaySound2D (Utilities|Select :Index (Variables|Default|GetProjectileType) :CT_None "/Game/Sound/Placeholder_Sounds/S_RedProjectileWallHit.S_RedProjectileWallHit" :CT_Red "/Game/Sound/Placeholder_Sounds/S_RedProjectileWallHit.S_RedProjectileWallHit" :CT_Blue "/Game/Sound/Placeholder_Sounds/S_BlueProjectileWallHit.S_BlueProjectileWallHit") 1.0 1.0 0.0 0 0))

(fn ConstructionScript
  (Variables|/Script/Engine.ProjectileMovementComponent|SetInitialSpeed (Variables|Default|GetEditorProjectileComponent) (* (Variables|/Script/Engine.ProjectileMovementComponent|GetInitialSpeed (Variables|Default|GetEditorProjectileComponent)) (Variables|Default|GetSpeedMultiplier))))

(fn HandleMismatchingHit
  (params (Enemy :type Actor%20Object%20Reference)))

(fn HandleMatchingHit
  (params (Enemy :type Actor%20Object%20Reference)))

(fn SpawnExplosion
  (bind _asbp_player_character (Utilities|Casting|CastToBP_PlayerCharacter (Variables|Default|GetPlayerOwner)))
  (LocalVariables|SetPlayerOwnerBP _asbp_player_character)
  (Game|SpawnActorfromClass "/Game/Gameplay/Blueprints/Combat/SpecialMechanics/Explosion/BP_ExplosionBase.BP_ExplosionBase_C" (Transformation|GetActorTransform) "Undefined" 0 (Variables|Default|GetProjectileType) (* (Class|ProjectileBase|GetDamage) 2.3) (LocalVariables|GetPlayerOwnerBP) (Variables|Default|GetChargeFraction) 0))

(fn HandleEnemyHit
  (params (Enemy :type BP%20Enemy%20Base%20Object%20Reference) (ColorMatch :type Boolean) (Damage :type Float%20%28single-precision%29))
  ;[1 1 1] Check Head
  (if (Class|PrimitiveComponent|IsOverlappingComponent (Variables|/Game/Characters/NPC/Blueprints/BP_EnemyBase.BP_EnemyBase_C|GetHeadSphere Enemy) (Variables|Default|GetEditorSphereComponent))
    (LocalVariables|SetEnemyHitLocation "EHT_Head")
    (else
      ;[1 1 1] Check Chest
      (if (Class|PrimitiveComponent|IsOverlappingComponent (Variables|/Game/Characters/NPC/Blueprints/BP_EnemyBase.BP_EnemyBase_C|GetChestBox Enemy) (Variables|Default|GetEditorSphereComponent))
        (LocalVariables|SetEnemyHitLocation "EHT_Chest")
        (else
          ;[1 1 1] Check Legs
          (if (Class|PrimitiveComponent|IsOverlappingComponent (Variables|/Game/Characters/NPC/Blueprints/BP_EnemyBase.BP_EnemyBase_C|GetLegBoxRight Enemy) (Variables|Default|GetEditorSphereComponent))
            (LocalVariables|SetEnemyHitLocation "EHT_LegRight")
            (elif (Class|PrimitiveComponent|IsOverlappingComponent (Variables|/Game/Characters/NPC/Blueprints/BP_EnemyBase.BP_EnemyBase_C|GetLegBoxLeft Enemy) (Variables|Default|GetEditorSphereComponent))
              (LocalVariables|SetEnemyHitLocation "EHT_LegLeft")
              (else
                ;[1 1 1] Unknown
                (LocalVariables|SetEnemyHitLocation "EHT_Unknown"))))))))
  (Utilities|FlowControl|Sequence
    (:then_0
      ;[1 1 1] Check Color Match
      (if ColorMatch
        (LocalVariables|SetFinalDamage Damage)
        ;[1 1 1] Projectile Color Match
        (switch Utilities|FlowControl|Switch|SwitchonEEnemyHitTypes (LocalVariables|GetEnemyHitLocation)
          (:EHT_Unknown
            (Development|PrintString "Warning! Unknown Enemy Hit Location" true true "(R=1.000000,G=0.000000,B=0.025391,A=1.000000)" 1e+02))
          (:EHT_Head
            ;;[1 1 1] Set Headshot Damage
            (LocalVariables|SetFinalDamage (* Damage 2.0))
            (Game|Damage|ApplyDamage Enemy (LocalVariables|GetFinalDamage) 0 (Variables|Default|GetPlayerOwner) :!label _label)
            (CallFunction|HandleMatchingHit)
            (Audio|PlaySound2D "/Game/Sound/Placeholder_Sounds/S_Matching_hit.S_Matching_hit" 1.0 1.0 0.0 0 0))
          (:EHT_Chest
            (goto _label))
          (:EHT_LegLeft
            ;;[1 1 1] Set Legshot Damage
            (LocalVariables|SetFinalDamage (* Damage 0.5) :!label _label_2)
            (Default|Slowed Enemy)
            (goto _label))
          (:EHT_LegRight
            (goto _label_2)))
        (else
          ;[1 1 1] Projectile Color Mismatch
          (Default|EmpowerEnemy Enemy Damage)
          (CallFunction|HandleMismatchingHit Enemy)
          (Audio|PlaySound2D "/Game/Sound/Placeholder_Sounds/S_Mismatching_hit.S_Mismatching_hit" 1.0 1.0 0.0 0 0))))
    (:then_1
      ;[1 1 1] Callback for enemy
      (Default|OnProjectileHit Enemy ColorMatch self (LocalVariables|GetEnemyHitLocation)))))