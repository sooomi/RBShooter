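; BP_ExplosionBase is a short-lived, color-coded explosion that grows every tick and destroys itself after one second.
; Each tick it deals frame-scaled damage, credited to the player, to overlapping BP_EnemyBase actors whose type matches its color, or to all when IgnoreColor is set.
; Mismatched enemies are instead stunned and empowered by the same amount.
; An older one-time, on-enter damage graph remains but never runs.
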(event EventBeginPlay
  ;[1 1 1] Destroy explosion
  (Utilities|FlowControl|Delay 1.0)
  (Actor|DestroyActor))

(event EventTick
  (params (DeltaSeconds :type Float%20%28single-precision%29))
  (bind _explosiondamage (Variables|Default|GetExplosionDamage))
  (bind _returnvalue (* _explosiondamage DeltaSeconds))
  (Utilities|FlowControl|Sequence
    (:then_0
      ;[1 1 1] Damage over time
      (for _array_element (Collision|GetOverlappingActors 0 :!class /Script/Engine.Actor)
        (if (Utilities|ClassIsChildOf (Utilities|GetClass _array_element) "/Game/Characters/NPC/Blueprints/BP_EnemyBase.BP_EnemyBase_C")
          (bind _asbp_enemy_base (Utilities|Casting|CastToBP_EnemyBase _array_element))
          (if (or (Utilities|Enum|Equal(Enum) (Variables|Default|GetColor) (Variables|/Script/RBShooter.Enemy|GetEnemyType _asbp_enemy_base)) (Variables|Default|GetIgnoreColor))
            (Game|Damage|ApplyDamage _array_element _returnvalue 0 (Game|GetPlayerCharacter 0))
            (else
              (Default|Stun _asbp_enemy_base 0.5)
              (Default|EmpowerEnemy _asbp_enemy_base _returnvalue))))))
    (:then_1
      ;[1 1 1] Swelling explosion
      (Transformation|SetActorScale3D (+ (Transformation|GetActorScale3D) (* DeltaSeconds 1.5))))))

(fn ConstructionScript)