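; BP_EnemyMagnetEffect is a timed magnet effect actor that links overlapping enemies of its color, or any color if unset, with lightning beams.
; Overlaps spawn color-matched beam emitters, tracked in a map to their enemy and removed on end overlap or expiry.
; Construction tints the sphere, and a timeline animates its displacement and distortion.
; An attraction flag turns on after a short delay; no pull logic is here.
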(event Custom|LifetimeExpired
  ;[1 1 1] Destroy all emitters then destroy self
  (bind _keys (Utilities|Map|Keys (Variables|Default|GetSpawnedLightningEmitters)))
  (for _array_element _keys
    (Components|DestroyComponent _array_element)
    (Utilities|Map|Remove (Variables|Default|GetSpawnedLightningEmitters) _array_element))
  (Actor|DestroyActor)
  (Utilities|Map|Clear (Variables|Default|GetSpawnedLightningEmitters)))

(event EventBeginPlay
  (Utilities|FlowControl|Sequence
    (:then_0
      ;[1 1 1] Create Timer Handle for duration
      (bind _returnvalue (Utilities|Time|SetTimerbyEvent (EventDispatchers|CreateEvent :!event Custom|LifetimeExpired) (Variables|Default|GetDuration)))
      (Variables|Default|SetLifetimeTimerHandle _returnvalue))
    (:then_1
      (|HandleSphereTimeline))
    (:then_2
      (Variables|Default|SetbIsAttractingEnemies false)
      (Utilities|FlowControl|Delay 0.25)
      (Variables|Default|SetbIsAttractingEnemies true))))

(event Collision|EventActorBeginOverlap
  (params (OtherActor :type Actor%20Object%20Reference))
  ;[1 1 1] Check if Other Actor is an enemy and that its color matches this color
  (if (Utilities|ClassIsChildOf (Utilities|GetClass OtherActor) "/Game/Characters/NPC/Blueprints/BP_EnemyBase.BP_EnemyBase_C")
    (bind _asbp_enemy_base (Utilities|Casting|CastToBP_EnemyBase OtherActor))
    (if (or (Utilities|Enum|Equal(Enum) (Variables|/Script/RBShooter.Enemy|GetEnemyType _asbp_enemy_base) (Variables|Default|GetEnemyType)) (Utilities|Enum|Equal(Enum) (Variables|Default|GetEnemyType) "CT_None"))
      (CallFunction|SpawnLightningEmitter _asbp_enemy_base) ; Spawn Lightning Emitter
    )))

(event Collision|EventActorEndOverlap
  (params (OtherActor :type Actor%20Object%20Reference))
  ;[1 1 1] Find emitter associated with Other Actor and destroy it
  (bind _keys (Utilities|Map|Keys (Variables|Default|GetSpawnedLightningEmitters)))
  (for _array_element _keys
    (if (and (== (.Value (Utilities|Map|Find (Variables|Default|GetSpawnedLightningEmitters) _array_element)) OtherActor) (.ReturnValue (Utilities|Map|Find (Variables|Default|GetSpawnedLightningEmitters) _array_element)))
      (Components|DestroyComponent _array_element)
      (Utilities|Map|Remove (Variables|Default|GetSpawnedLightningEmitters) _array_element))))

(fn ConstructionScript
  (CallFunction|UpdateSphereColor))

(fn SpawnLightningEmitter
  (params (EnemyActor :type BP%20Enemy%20Base%20Object%20Reference))
  ;[1 1 1] Spawn Emitter & add to map together with Enemy Actor
  (bind _returnvalue (Effects|SpawnEmitteratLocation "/Game/Effects/Particles/P_Lightning.P_Lightning" (Transformation|GetActorLocation)))
  (bind _output_get (LocalVariables|SetLightningEmitter _returnvalue))
  (Utilities|Map|Add (Variables|Default|GetSpawnedLightningEmitters) _output_get EnemyActor)
  ;[1 0.6964 0.375] Set Lightning Beam Source & Target
  (Effects|Components|ParticleSystem|SetActorParameter (LocalVariables|GetLightningEmitter) "LightningTarget" EnemyActor)
  (Effects|Components|ParticleSystem|SetActorParameter (LocalVariables|GetLightningEmitter) "LightningSource" self)
  ;[0.5052 1 0.9793] Set Particle Color
  (switch Utilities|FlowControl|Switch|SwitchonEColorTypes (Variables|/Script/RBShooter.Enemy|GetEnemyType EnemyActor)
    (:CT_None
      (Effects|Components|ParticleSystem|SetColorParameter (LocalVariables|GetLightningEmitter) "LightningColor" "(R=1.000000,G=0.000000,B=0.023868,A=1.000000)" :!label _label))
    (:CT_Red
      (goto _label))
    (:CT_Blue
      (Effects|Components|ParticleSystem|SetColorParameter (LocalVariables|GetLightningEmitter) "LightningColor" "(R=0.000000,G=0.603337,B=1.000000,A=1.000000)"))))

(fn UpdateSphereColor
  (switch Utilities|FlowControl|Switch|SwitchonEColorTypes (Variables|Default|GetEnemyType)
    (:CT_Red
      (Rendering|Material|SetVectorParameterValueonMaterials (Variables|Default|GetSphere) "EmissiveColor" (Math|Conversions|ToVector(LinearColor) "(R=1.000000,G=0.000000,B=0.097409,A=1.000000)")))
    (:CT_Blue
      (Rendering|Material|SetVectorParameterValueonMaterials (Variables|Default|GetSphere) "EmissiveColor" (Math|Conversions|ToVector(LinearColor) "(R=0.000000,G=0.464699,B=1.000000,A=1.000000)")))))