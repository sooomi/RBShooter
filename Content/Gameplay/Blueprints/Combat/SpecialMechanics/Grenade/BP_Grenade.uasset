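; Thrown color-typed grenade that pulls in enemies with a magnet effect, then explodes.
; On BeginPlay it launches its physics sphere with an upward boost, then activates once, after a delay or on hitting an enemy.
; Activation hides the sphere, spawns the magnet just above it and, late in the magnet's duration, spawns a red or blue explosion and destroys the actor.
; Hard impacts also play a sound.
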(event EventBeginPlay
  (Physics|SetPhysicsLinearVelocity (Variables|Default|GetSphere) (+ (* (Variables|Default|GetThrowDirection) (Variables|Default|GetThrowForce)) "0, 0,250.000000") false "None")
  (Utilities|FlowControl|Delay (Variables|Default|GetActivationDelay))
  (if (not (Variables|Default|GetHasActivated))
    (Rendering|SetVisibility (Variables|Default|GetSphere) false false)
    (Variables|Default|SetMagnetLocation (+ (Transformation|GetWorldLocation (Variables|Default|GetSphere)) "0, 0,100.000000"))
    (Variables|Default|SetHasActivated true)
    (Game|SpawnActorfromClass "/Game/Gameplay/Blueprints/Combat/SpecialMechanics/Magnet/BP_EnemyMagnetEffect.BP_EnemyMagnetEffect_C" (Math|Transform|MakeTransform (Variables|Default|GetMagnetLocation) (Transformation|GetWorldRotation (Variables|Default|GetSphere))) "Undefined" 0 (Variables|Default|GetMagnetDuration) (Variables|Default|GetColorType) 3.0 5.0 0)
    (Utilities|FlowControl|Delay (* (Variables|Default|GetMagnetDuration) 0.8))
    (switch Utilities|FlowControl|Switch|SwitchonEColorTypes (Variables|Default|GetColorType)
      (:CT_Red
        (bind _returnvalue (Game|SpawnActorfromClass "/Game/Gameplay/Blueprints/Combat/SpecialMechanics/Explosion/BP_ExplosionRed1.BP_ExplosionRed1_C" (Math|Transform|MakeTransform (Variables|Default|GetMagnetLocation) (Transformation|GetWorldRotation (Variables|Default|GetSphere)) "3.000000,3.000000,3.000000") "Undefined" 0 (Variables|Default|GetColorType) 0))
        (Variables|/Game/Gameplay/Blueprints/Combat/SpecialMechanics/Explosion/BP_ExplosionBase.BP_ExplosionBase_C|SetExplosionDamage _returnvalue 3.0))
      (:CT_Blue
        (bind _returnvalue_2 (Game|SpawnActorfromClass "/Game/Gameplay/Blueprints/Combat/SpecialMechanics/Explosion/BP_ExplosionBlue1.BP_ExplosionBlue1_C" (Math|Transform|MakeTransform (Variables|Default|GetMagnetLocation) (Transformation|GetWorldRotation (Variables|Default|GetSphere)) "3.000000,3.000000,3.000000") "Undefined" 0 (Variables|Default|GetColorType) 0))
        (Variables|/Game/Gameplay/Blueprints/Combat/SpecialMechanics/Explosion/BP_ExplosionBase.BP_ExplosionBase_C|SetExplosionDamage _returnvalue_2 3.0)))
    (Actor|DestroyActor)))

(event Collision|EventHit
  (params (MyComp :type Primitive%20Component%20Object%20Reference) (Other :type Actor%20Object%20Reference) (OtherComp :type Primitive%20Component%20Object%20Reference) (bSelfMoved :type Boolean) (HitLocation :type Vector :default "0, 0, 0") (HitNormal :type Vector :default "0, 0, 0") (NormalImpulse :type Vector :default "0, 0, 0") (Hit :type Hit%20Result%20Structure%20%28by%20ref%29))
  (Utilities|FlowControl|Sequence
    (:then_0
      (if (Utilities|ClassIsChildOf (Utilities|GetClass Other) "/Game/Characters/NPC/Blueprints/BP_EnemyBase.BP_EnemyBase_C")
        (if (not (Variables|Default|GetHasActivated))
          (Rendering|SetVisibility (Variables|Default|GetSphere) false false)
          (Variables|Default|SetMagnetLocation (+ (Transformation|GetWorldLocation (Variables|Default|GetSphere)) "0, 0,100.000000"))
          (Variables|Default|SetHasActivated true)
          (Game|SpawnActorfromClass "/Game/Gameplay/Blueprints/Combat/SpecialMechanics/Magnet/BP_EnemyMagnetEffect.BP_EnemyMagnetEffect_C" (Math|Transform|MakeTransform (Variables|Default|GetMagnetLocation) (Transformation|GetWorldRotation (Variables|Default|GetSphere))) "Undefined" 0 (Variables|Default|GetMagnetDuration) (Variables|Default|GetColorType) 3.0 5.0 0)
          (Utilities|FlowControl|Delay (* (Variables|Default|GetMagnetDuration) 0.8))
          (switch Utilities|FlowControl|Switch|SwitchonEColorTypes (Variables|Default|GetColorType)
            (:CT_Red
              (bind _returnvalue (Game|SpawnActorfromClass "/Game/Gameplay/Blueprints/Combat/SpecialMechanics/Explosion/BP_ExplosionRed1.BP_ExplosionRed1_C" (Math|Transform|MakeTransform (Variables|Default|GetMagnetLocation) (Transformation|GetWorldRotation (Variables|Default|GetSphere)) "3.000000,3.000000,3.000000") "Undefined" 0 (Variables|Default|GetColorType) 0))
              (Variables|/Game/Gameplay/Blueprints/Combat/SpecialMechanics/Explosion/BP_ExplosionBase.BP_ExplosionBase_C|SetExplosionDamage _returnvalue 3.0))
            (:CT_Blue
              (bind _returnvalue_2 (Game|SpawnActorfromClass "/Game/Gameplay/Blueprints/Combat/SpecialMechanics/Explosion/BP_ExplosionBlue1.BP_ExplosionBlue1_C" (Math|Transform|MakeTransform (Variables|Default|GetMagnetLocation) (Transformation|GetWorldRotation (Variables|Default|GetSphere)) "3.000000,3.000000,3.000000") "Undefined" 0 (Variables|Default|GetColorType) 0))
              (Variables|/Game/Gameplay/Blueprints/Combat/SpecialMechanics/Explosion/BP_ExplosionBase.BP_ExplosionBase_C|SetExplosionDamage _returnvalue_2 3.0)))
          (Actor|DestroyActor))))
    (:then_1
      (if (> (Math|Vector|VectorLength NormalImpulse) 1.3e+03)
        (Audio|SpawnSoundatLocation "/Game/Characters/Player/Sound/steps_06.steps_06" HitLocation "0, 0, 0" 1.0 1.0 0.0 0 0)))))

(fn ConstructionScript)