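; Short-lived force-push actor that knocks back BP_EnemyBase enemies entering it and destroys itself after one second.
; On overlap it records the enemy in AffectedActors and launches it, but the repeat-hit check receives no actor, so it does not match recorded enemies.
; Launch direction radiates from a point below the actor to add lift, with strength scaled by sphere radius minus distance from that point, overriding current velocity.
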(event EventBeginPlay
  (Utilities|FlowControl|Delay 1.0)
  (Actor|DestroyActor))

(event Collision|EventActorBeginOverlap
  (params (OtherActor :type Actor%20Object%20Reference))
  (bind _asbp_enemy_base (Utilities|Casting|CastToBP_EnemyBase OtherActor))
  (if (Utilities|IsValid _asbp_enemy_base)
    (if (not (CallFunction|HasActorBeenAffectedBefore))
      (Utilities|Array|Add (Variables|Default|GetAffectedActors) _asbp_enemy_base)
      (CallFunction|PushBackEnemy _asbp_enemy_base))))

(event EventTick
  (params (DeltaSeconds :type Float%20%28single-precision%29)))

(fn ConstructionScript)

(fn HasActorBeenAffectedBefore
  (params (Actor :type Actor%20Object%20Reference))
  (for _array_element (Variables|Default|GetAffectedActors)
    (if (== _array_element Actor)
      (return true)))
  (return false))

(fn PushBackEnemy
  (params (enemy :type BP%20Enemy%20Base%20Object%20Reference))
  (bind _returnvalue (Transformation|GetActorLocation))
  (bind _returnvalue_2 (Transformation|GetActorLocation enemy))
  (bind _returnvalue_3 (+ _returnvalue "0, 0,-200.000000"))
  (bind _returnvalue_4 (- _returnvalue_2 _returnvalue_3))
  (Character|LaunchCharacter enemy (* (Math|Vector|Normalize _returnvalue_4) (* (- (Components|Sphere|GetScaledSphereRadius (Variables|Default|GetSphereCollider)) (Math|Vector|VectorLength _returnvalue_4)) 5e+01)) true true))