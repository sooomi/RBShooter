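; BP_ExplosionBase is a color-typed explosion that affects enemies caught in its radius once, when it spawns.
; On BeginPlay it gathers BP_EnemyBase pawns overlapping its sphere collider, damages those matching its ColorType on behalf of PlayerOwner, and stuns and empowers the rest.
; The construction script tints the particle system by ColorType.
; It also plays a charge-shot sound at the world origin and destroys itself after a short delay.
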(event EventBeginPlay
  (bind _spherecollider (Variables|Default|GetSphereCollider))
  (Utilities|FlowControl|Sequence
    (:then_0
      ;[1 1 1] Damage Overlapping Enemies
      (bind _outactors (Collision|ComponentOverlapActors _spherecollider (Transformation|GetWorldTransform _spherecollider) (Utilities|Array|MakeArray "ObjectTypeQuery3") "/Game/Characters/NPC/Blueprints/BP_EnemyBase.BP_EnemyBase_C"))
      (for _array_element _outactors
        (bind _asbp_enemy_base (Utilities|Casting|CastToBP_EnemyBase _array_element))
        (CallFunction|DamageEnemy _asbp_enemy_base)))
    (:then_1
      ;[1 1 1] Destroy explosion
      (Audio|PlaySoundatLocation "/Game/Sound/Placeholder_Sounds/S_Chargeshot.S_Chargeshot" "0, 0, 0" "0, 0, 0" 1.0 1.0 0.0 0 0 0)
      (Utilities|FlowControl|Delay 3.0)
      (Actor|DestroyActor))))

(fn ConstructionScript
  (Effects|Components|ParticleSystem|SetColorParameter (Variables|Default|GetParticleSystem) "Color" (Utilities|Select :Index (Variables|Default|GetColorType) :CT_None "(R=1.000000,G=1.000000,B=1.000000,A=1.000000)" :CT_Red "(R=1.000000,G=0.000000,B=0.014359,A=1.000000)" :CT_Blue "(R=0.000000,G=0.538799,B=1.000000,A=1.000000)")))

(fn DamageEnemy
  (params (Enemy :type BP%20Enemy%20Base%20Object%20Reference))
  (if (Utilities|Enum|Equal(Enum) (Variables|/Script/RBShooter.Enemy|GetEnemyType Enemy) (Variables|Default|GetColorType))
    (Game|Damage|ApplyDamage Enemy (Variables|Default|GetDamage) 0 (Variables|Default|GetPlayerOwner))
    (else
      ;[1 1 1] Stun & Empower
      (Default|Stun Enemy 0.5)
      (Default|EmpowerEnemy Enemy 1.0))))