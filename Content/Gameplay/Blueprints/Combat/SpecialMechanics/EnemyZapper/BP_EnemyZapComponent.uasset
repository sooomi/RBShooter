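; Enemy zap component that fires a lightning beam at an enemy and kills it after a delay.
; The Zap event spawns a lightning beam particle on the zapper, running from a given source point to the enemy and tinted by the enemy's color type.
; After the duration, if the enemy is still valid, it destroys the beam and kills the enemy, crediting the zapper's owning player.
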(event Custom|Zap
  (params (EnemyZapper :type BP%20Enemy%20Zapper%20Object%20Reference) (Enemy :type BP%20Enemy%20Base%20Object%20Reference) (Duration :type Float%20%28single-precision%29) (LightningSource :type Vector))
  (bind _emitter (CallFunction|SpawnLightningEmitter EnemyZapper Enemy LightningSource))
  (Utilities|FlowControl|Delay Duration)
  (if (Utilities|IsValid Enemy)
    (Components|DestroyComponent _emitter)
    (Class|HealthComponent|Kill (Variables|/Game/Characters/NPC/Blueprints/BP_EnemyBase.BP_EnemyBase_C|GetHealth Enemy) (Variables|/Game/Gameplay/Blueprints/Combat/SpecialMechanics/EnemyZapper/BP_EnemyZapper.BP_EnemyZapper_C|GetPlayerOwner EnemyZapper))))

(event EventBeginPlay)

(event EventTick
  (params (DeltaSeconds :type Float%20%28single-precision%29)))

(fn SpawnLightningEmitter
  (params (EnemyZapper :type BP%20Enemy%20Zapper%20Object%20Reference) (Enemy :type BP%20Enemy%20Base%20Object%20Reference) (LightningSource :type Vector))
  (bind _returnvalue (Effects|SpawnEmitterAttached "/Game/Gameplay/Particles/EnemyZap/P_EnemyZapLightning.P_EnemyZapLightning" (Variables|/Game/Gameplay/Blueprints/Combat/SpecialMechanics/EnemyZapper/BP_EnemyZapper.BP_EnemyZapper_C|GetDefaultSceneRoot EnemyZapper) "None" (Transformation|GetActorLocation Enemy) "0, 0, 0" "1.000000,1.000000,1.000000" "KeepWorldPosition"))
  (LocalVariables|SetSpawnedEmitter _returnvalue)
  (Class|ParticleSystemComponent|SetBeamSourcePoint (LocalVariables|GetSpawnedEmitter) 0 LightningSource)
  (Effects|Components|ParticleSystem|SetActorParameter (LocalVariables|GetSpawnedEmitter) "LightningTarget" Enemy)
  (Effects|Components|ParticleSystem|SetColorParameter (LocalVariables|GetSpawnedEmitter) "LightningColor" (Utilities|Select :Index (Variables|/Script/RBShooter.Enemy|GetEnemyType Enemy) :CT_None "(R=1.000000,G=1.000000,B=1.000000,A=1.000000)" :CT_Red "(R=1.000000,G=0.000000,B=0.008760,A=1.000000)" :CT_Blue "(R=0.000000,G=0.421747,B=1.000000,A=1.000000)"))
  (return (LocalVariables|GetSpawnedEmitter)))