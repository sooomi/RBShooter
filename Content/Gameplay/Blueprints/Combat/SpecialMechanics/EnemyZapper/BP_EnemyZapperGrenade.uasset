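; Thrown grenade actor that deploys a BP_EnemyZapper where it lands or strikes.
; On BeginPlay it plays a whoosh sound and launches its physics sphere along ThrowDirection scaled by ThrowForce.
; On hit it spawns the zapper at the impact location, passes on ColorType and PlayerOwner, then destroys itself.
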(event EventBeginPlay
  (Audio|SpawnSound2D "/Game/Sound/Placeholder_Sounds/S_GrenadeWosh.S_GrenadeWosh" 1.0 1.0 0.0 0)
  (Physics|SetPhysicsLinearVelocity (Variables|Default|GetSphere) (* (Variables|Default|GetThrowDirection) (Variables|Default|GetThrowForce)) false "None"))

(event EventTick
  (params (DeltaSeconds :type Float%20%28single-precision%29)))

(event Collision|EventHit
  (params (MyComp :type Primitive%20Component%20Object%20Reference) (Other :type Actor%20Object%20Reference) (OtherComp :type Primitive%20Component%20Object%20Reference) (bSelfMoved :type Boolean) (HitLocation :type Vector :default "0, 0, 0") (HitNormal :type Vector :default "0, 0, 0") (NormalImpulse :type Vector :default "0, 0, 0") (Hit :type Hit%20Result%20Structure%20%28by%20ref%29))
  (Game|SpawnActorfromClass "/Game/Gameplay/Blueprints/Combat/SpecialMechanics/EnemyZapper/BP_EnemyZapper.BP_EnemyZapper_C" (Math|Transform|MakeTransform HitLocation) "Undefined" 0 (Variables|Default|GetColorType) (Variables|Default|GetPlayerOwner) 1e+01 0)
  (Actor|DestroyActor))

(fn ConstructionScript)