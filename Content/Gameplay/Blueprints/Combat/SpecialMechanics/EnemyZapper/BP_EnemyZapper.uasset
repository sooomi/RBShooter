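; BP_EnemyZapper is a timed combat actor that zaps enemies overlapping it, then destroys itself after Duration.
; On overlap, it filters BP_EnemyBase actors by ColorType against EnemyType, with no color matching every enemy.
; Each valid hit adds a new zap component to the zapper, which runs a short zap on that enemy.
; The construction script tints the sphere's emissive material to match ColorType.
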(event EventBeginPlay
  (Utilities|FlowControl|Delay (Variables|Default|GetDuration))
  (Actor|DestroyActor))

(event Collision|EventActorBeginOverlap
  (params (OtherActor :type Actor%20Object%20Reference))
  (bind _asbp_enemy_base (Utilities|Casting|CastToBP_EnemyBase OtherActor))
  (if (Utilities|IsValid _asbp_enemy_base)
    (if (or (Utilities|Enum|Equal(Enum) (Variables|Default|GetColorType) "CT_None") (Utilities|Enum|Equal(Enum) (Variables|/Script/RBShooter.Enemy|GetEnemyType _asbp_enemy_base) (Variables|Default|GetColorType)))
      (bind _returnvalue (AddComponent|AddBPEnemyZapComponent))
      (Default|Zap _returnvalue self _asbp_enemy_base 0.5))))

(fn ConstructionScript
  (CallFunction|UpdateSphereColor))

(fn UpdateSphereColor
  (Rendering|Material|SetVectorParameterValueonMaterials (Variables|Default|GetSphere) "EmissiveColor" (Math|Conversions|ToVector(LinearColor) (Utilities|Select :Index (Variables|Default|GetColorType) :CT_None "(R=1.000000,G=1.000000,B=1.000000,A=1.000000)" :CT_Red "(R=1.000000,G=0.000000,B=0.058392,A=1.000000)" :CT_Blue "(R=0.000000,G=0.795079,B=1.000000,A=1.000000)"))))