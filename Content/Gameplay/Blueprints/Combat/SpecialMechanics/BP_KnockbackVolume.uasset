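; A short-lived knockback volume that stuns and launches enemies, styled as a shout with the FosRoDoh sound.
; On BeginPlay it plays the sound in 2D and destroys itself after a brief delay.
; Any overlapping BP_EnemyBase child is stunned and launched along the player character's forward vector scaled by KnockbackAmount, plus a fixed upward boost.
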(event EventBeginPlay
  (Audio|PlaySound2D "/Game/Sound/Placeholder_Sounds/S_FosRoDoh.S_FosRoDoh" 1.0 1.0 0.0 0 0)
  (Utilities|FlowControl|Delay 0.3)
  (Actor|DestroyActor))

(event Collision|EventActorBeginOverlap
  (params (OtherActor :type Actor%20Object%20Reference))
  (if (Utilities|ClassIsChildOf (Utilities|GetClass OtherActor) "/Game/Characters/NPC/Blueprints/BP_EnemyBase.BP_EnemyBase_C")
    (bind _asbp_enemy_base (Utilities|Casting|CastToBP_EnemyBase OtherActor))
    (Default|Stun _asbp_enemy_base 1.0)
    (Character|LaunchCharacter _asbp_enemy_base (+ (* (Transformation|GetActorForwardVector (Game|GetPlayerCharacter 0)) (Variables|Default|GetKnockback%20Amount)) "0, 0,500.000000") false false)))

(event EventTick
  (params (DeltaSeconds :type Float%20%28single-precision%29)))

(fn ConstructionScript)