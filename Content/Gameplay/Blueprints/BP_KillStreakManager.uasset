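; Kill-streak manager that rewards consecutive kills of the same enemy color with bonus weapon damage.
; It binds to the game mode's enemy-death and wave-completed events, though the wave handler is empty.
; A color change resets the count and red/blue damage; count milestones raise the matching color's damage or, at 20, generic damage.
; Red's second milestone compares constants and never fires, and damage values print as debug output.
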(event Custom|EnemyDied
  (params (Enemy :type BP%20Enemy%20Base%20Object%20Reference) (Killer :type Actor%20Object%20Reference))
  (bind _playercharacter (Variables|Default|GetPlayerCharacter))
  (bind _playercharacter_2 (Variables|Default|GetPlayerCharacter))
  (bind _playercharacter_3 (Variables|Default|GetPlayerCharacter))
  (bind _playercharacter_4 (Variables|Default|GetPlayerCharacter))
  (bind _enemytype (Variables|/Script/RBShooter.Enemy|GetEnemyType Enemy))
  (bind _playercharacter_5 (Variables|Default|GetPlayerCharacter))
  (bind _playercharacter_6 (Variables|Default|GetPlayerCharacter))
  (bind _weaponactor (Variables|/Script/RBShooter.PlayerCharacter|GetWeaponActor _playercharacter_3))
  ;[1 1 1] Example
  (if (Utilities|Enum|Equal(Enum) _enemytype (Variables|Default|GetCurrentStreakColor))
    _
    (else
      (Variables|Default|SetCurrentStreakColor _enemytype)
      (Variables|Default|SetNumber%20Of%20Kills 0)
      (Variables|/Script/RBShooter.Weapon|SetDamageBlue _weaponactor 0.0)
      (Variables|/Script/RBShooter.Weapon|SetDamageRed _weaponactor 0.0)))
  (bind _output_get (Variables|Default|SetNumber%20Of%20Kills (+ (Variables|Default|GetNumber%20Of%20Kills) 1)))
  (if (Utilities|Enum|Equal(Enum) "CT_Red" (Variables|Default|GetCurrentStreakColor))
    (if (== (+ (Variables|Default|GetNumber%20Of%20Kills) 1) 5)
      (bind _output_get_2 (Variables|/Script/RBShooter.Weapon|SetDamageRed (Variables|/Script/RBShooter.PlayerCharacter|GetWeaponActor _playercharacter_2) (+ (Variables|/Script/RBShooter.Weapon|GetDamageRed (Variables|/Script/RBShooter.PlayerCharacter|GetWeaponActor _playercharacter_2)) 1.0)))
      (else
        (Development|PrintString (Utilities|String|ToString(Float) _output_get_2))
        (if (== 0 10)
          (Variables|/Script/RBShooter.Weapon|SetDamageRed (Variables|/Script/RBShooter.PlayerCharacter|GetWeaponActor _playercharacter_6) (+ (Variables|/Script/RBShooter.Weapon|GetDamageRed (Variables|/Script/RBShooter.PlayerCharacter|GetWeaponActor _playercharacter_6)) 1.0))
          (else
            (if (== _output_get 20) :!label _label
              (Variables|/Script/RBShooter.Weapon|SetDamageGeneric (Variables|/Script/RBShooter.PlayerCharacter|GetWeaponActor _playercharacter_5) (+ (Variables|/Script/RBShooter.Weapon|GetDamageGeneric (Variables|/Script/RBShooter.PlayerCharacter|GetWeaponActor _playercharacter_5)) 1.0)))))))
    (elif (== (+ (Variables|Default|GetNumber%20Of%20Kills) 1) 5)
      (bind _output_get_3 (Variables|/Script/RBShooter.Weapon|SetDamageBlue (Variables|/Script/RBShooter.PlayerCharacter|GetWeaponActor _playercharacter_4) (+ (Variables|/Script/RBShooter.Weapon|GetDamageBlue (Variables|/Script/RBShooter.PlayerCharacter|GetWeaponActor _playercharacter_4)) 1.0)))
      (else
        (Development|PrintString (Utilities|String|ToString(Float) _output_get_3))
        (if (== (+ (Variables|Default|GetNumber%20Of%20Kills) 1) 10)
          (Variables|/Script/RBShooter.Weapon|SetDamageBlue (Variables|/Script/RBShooter.PlayerCharacter|GetWeaponActor _playercharacter) (+ (Variables|/Script/RBShooter.Weapon|GetDamageBlue (Variables|/Script/RBShooter.PlayerCharacter|GetWeaponActor _playercharacter)) 1.0))
          (else
            (goto _label)))))))

(event Custom|WaveCompleted
  (params (WaveNumber :type Integer) (TimeLeft :type Float%20%28single-precision%29))
  ;[1 1 1] Example
)

(event EventBeginPlay
  (Utilities|FlowControl|Sequence
    (:then_0
      ;[1 1 1] Store reference to gamemode
      (bind _asbp_rbshooter_game_mode (Utilities|Casting|CastToBP_RBShooterGameMode (Game|GetGameMode)))
      (Variables|Default|SetGameMode _asbp_rbshooter_game_mode))
    (:then_1
      ;[1 1 1] Store reference to playercharacter
      (bind _asbp_player_character (Utilities|Casting|CastToBP_PlayerCharacter (Game|GetPlayerCharacter 0)))
      (Variables|Default|SetPlayerCharacter _asbp_player_character))
    (:then_2
      ;[1 1 1] Example
      (EventDispatchers|BindEventtoOnEnemyDiedBP (Variables|Default|GetGameMode) (delegate Custom|EnemyDied)))
    (:then_3
      ;[1 1 1] Example
      (EventDispatchers|BindEventtoOnWaveCompletedBP (Variables|Default|GetGameMode) (delegate Custom|WaveCompleted)))))

(event Collision|EventActorBeginOverlap
  (params (OtherActor :type Actor%20Object%20Reference)))

(event EventTick
  (params (DeltaSeconds :type Float%20%28single-precision%29)))

(fn ConstructionScript)