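; BP_PickUpHeal is a healing pickup that the player character collects by interacting with it.
; On interaction it notifies BP_PlayerCharacter and restores half of that character's missing health through its Health component, so the heal scales with the damage taken.
; It then plays a 2D heal sound, spawns a BP_HealEffect actor at its own transform and destroys itself.
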(event EventBeginPlay)

(event Collision|EventActorBeginOverlap
  (params (OtherActor :type Actor%20Object%20Reference))
  (|CallParentFunction OtherActor) ; This node is disabled and will not be called.\nDrag off pins to build functionality.
)

(event EventTick
  (params (DeltaSeconds :type Float%20%28single-precision%29)))

(event EventOnInteracted
  (params (InteractedObject :type Actor%20Object%20Reference))
  (bind _asbp_player_character (Utilities|Casting|CastToBP_PlayerCharacter InteractedObject))
  (Default|HealPickedUp _asbp_player_character)
  (Class|HealthComponent|AddHealth (Variables|/Game/Characters/Player/Blueprints/BP_PlayerCharacter.BP_PlayerCharacter_C|GetHealth _asbp_player_character) (/ (- (Variables|/Script/RBShooter.HealthComponent|GetMaxHealth (Variables|/Game/Characters/Player/Blueprints/BP_PlayerCharacter.BP_PlayerCharacter_C|GetHealth _asbp_player_character)) (Variables|/Script/RBShooter.HealthComponent|GetCurrentHealth (Variables|/Game/Characters/Player/Blueprints/BP_PlayerCharacter.BP_PlayerCharacter_C|GetHealth _asbp_player_character))) 2.0) 0)
  (Audio|PlaySound2D "/Game/Sound/Placeholder_Sounds/S_HealthAdded.S_HealthAdded" 5.0 1.0 0.0 0 0)
  (Game|SpawnActorfromClass "/Game/Effects/Blueprints/BP_HealEffect.BP_HealEffect_C" (Transformation|GetActorTransform) "Undefined" 0 0)
  (Actor|DestroyActor))

(fn ConstructionScript
  (|CallParentFunction))