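; BP_Dragonborn is a short-lived Niagara effect actor that feeds the player character's position and direction into its particle system, then destroys itself after three seconds.
; BeginPlay and every Tick run the same update, setting the User.PlayerDirection and User.PlayerLocation Niagara variables.
; Direction is the scaled unit vector from the actor root to the player's capsule.
; Location is the sum of both world positions, not the player's position alone.
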(event EventBeginPlay
  (bind _returnvalue (Game|GetPlayerCharacter 0))
  (bind _defaultsceneroot (Variables|Default|GetDefaultSceneRoot))
  (bind _niagara (Variables|Default|GetNiagara))
  (bind _returnvalue_2 (Actor|GetComponentbyClass _returnvalue "/Script/Engine.CapsuleComponent"))
  (bind _returnvalue_3 (Transformation|GetWorldLocation _defaultsceneroot))
  (bind _returnvalue_4 (Transformation|GetWorldLocation _returnvalue_2))
  (Utilities|FlowControl|Sequence
    (:then_0
      (Utilities|FlowControl|Delay 3.0)
      (Actor|DestroyActor))
    (:then_1
      (bind _output_get (Variables|Default|SetPlayerLocation (+ _returnvalue_3 _returnvalue_4)))
      (bind _output_get_2 (Variables|Default|SetPlayerDirection (Math|Vector|GetUnitDirection(Vector) _returnvalue_3 _returnvalue_4)))
      (Class|NiagaraComponent|SetNiagaraVariableVec3 _niagara "User.PlayerDirection" (* _output_get_2 1e+03))
      (Class|NiagaraComponent|SetNiagaraVariableVec3 _niagara "User.PlayerLocation" _output_get))))

(event Collision|EventActorBeginOverlap
  (params (OtherActor :type Actor%20Object%20Reference)))

(event EventTick
  (params (DeltaSeconds :type Float%20%28single-precision%29))
  (bind _returnvalue (Game|GetPlayerCharacter 0))
  (bind _defaultsceneroot (Variables|Default|GetDefaultSceneRoot))
  (bind _niagara (Variables|Default|GetNiagara))
  (bind _returnvalue_2 (Actor|GetComponentbyClass _returnvalue "/Script/Engine.CapsuleComponent"))
  (bind _returnvalue_3 (Transformation|GetWorldLocation _defaultsceneroot))
  (bind _returnvalue_4 (Transformation|GetWorldLocation _returnvalue_2))
  (bind _output_get (Variables|Default|SetPlayerLocation (+ _returnvalue_3 _returnvalue_4)))
  (bind _output_get_2 (Variables|Default|SetPlayerDirection (Math|Vector|GetUnitDirection(Vector) _returnvalue_3 _returnvalue_4)))
  (Class|NiagaraComponent|SetNiagaraVariableVec3 _niagara "User.PlayerDirection" (* _output_get_2 1e+03))
  (Class|NiagaraComponent|SetNiagaraVariableVec3 _niagara "User.PlayerLocation" _output_get))

(fn ConstructionScript)