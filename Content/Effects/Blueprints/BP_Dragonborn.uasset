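; BP_Dragonborn is a short-lived effect actor that feeds player-relative data to a Niagara system and destroys itself five seconds after BeginPlay.
; On BeginPlay and every Tick, it reads the position of player character 0 and computes the unit direction from itself toward that character.
; It writes the location and the direction, scaled by ParticleSpeed, to Niagara user vector parameters, so the effect can track the moving player.
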(event EventBeginPlay
  (bind _returnvalue (Game|GetPlayerCharacter 0))
  (bind _niagara (Variables|Default|GetNiagara))
  (bind _returnvalue_2 (Transformation|GetActorLocation _returnvalue))
  (Utilities|FlowControl|Sequence
    (:then_0
      ;[1 1 1] Destroy once done
      (Utilities|FlowControl|Delay 5.0)
      (Actor|DestroyActor))
    (:then_1
      ;[1 1 1] Send values to Niagara system
      (bind _output_get (Variables|Default|SetPlayerLocation _returnvalue_2))
      (bind _output_get_2 (Variables|Default|SetPlayerDirection (Math|Vector|GetUnitDirection(Vector) (Transformation|GetActorLocation) _returnvalue_2)))
      (Class|NiagaraComponent|SetNiagaraVariableVec3 _niagara "User.PlayerDirection" (* _output_get_2 (Variables|Default|GetParticle%20Speed)))
      (Class|NiagaraComponent|SetNiagaraVariableVec3 _niagara "User.PlayerLocation" _output_get))))

(event EventTick
  (params (DeltaSeconds :type Float%20%28single-precision%29))
  (bind _returnvalue (Game|GetPlayerCharacter 0))
  (bind _niagara (Variables|Default|GetNiagara))
  (bind _returnvalue_2 (Transformation|GetActorLocation _returnvalue))
  ;[1 1 1] Send values to Niagara system
  (bind _output_get (Variables|Default|SetPlayerLocation _returnvalue_2))
  (bind _output_get_2 (Variables|Default|SetPlayerDirection (Math|Vector|GetUnitDirection(Vector) (Transformation|GetActorLocation) _returnvalue_2)))
  (Class|NiagaraComponent|SetNiagaraVariableVec3 _niagara "User.PlayerDirection" (* _output_get_2 (Variables|Default|GetParticle%20Speed)))
  (Class|NiagaraComponent|SetNiagaraVariableVec3 _niagara "User.PlayerLocation" _output_get))

(fn ConstructionScript)