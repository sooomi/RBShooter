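; Actor component that drives a dissolve effect with a glowing edge flare on its owner's mesh materials.
; BeginPlay caches the owner's mesh component, which SetMesh can replace.
; ActivateEffect maps an inverted fraction to a dissolve target and optionally starts a flare, which FlareUp also triggers alone.
; Tick eases the dissolve toward its target and drives emissive and edge thickness through FlareCurve, writing scalar material parameters.
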(event EventBeginPlay
  ;[1 1 1] Store reference to owner's mesh component
  (bind _output_get (Variables|Default|SetMeshComponent (Actor|GetComponentbyClass (Components|GetOwner) "/Script/Engine.MeshComponent")))
  (if (Utilities|IsValid _output_get)
    (Rendering|Material|SetScalarParameterValueonMaterials (Variables|Default|GetMeshComponent) "DissolveFraction" 0.0)
    (Rendering|Material|SetScalarParameterValueonMaterials (Variables|Default|GetMeshComponent) "EmissiveAmount" (Variables|Default|GetEmissiveAmountDefault))
    (Rendering|Material|SetScalarParameterValueonMaterials (Variables|Default|GetMeshComponent) "EmissiveAmount" (Variables|Default|GetEdgeThicknessDefault))
    (else
      (Development|PrintString "MeshComponent is invalid in DissolveEffectComponent!" true true "(R=1.000000,G=0.000000,B=0.022203,A=1.000000)" 3e+01))))

(event EventTick
  (params (DeltaSeconds :type Float%20%28single-precision%29))
  ;[1 1 1] Update effect if active
  (if (Utilities|IsValid (Variables|Default|GetMeshComponent))
    (Utilities|FlowControl|Sequence
      (:then_0
        ;[1 1 1] Update dissolve amount
        (if (Variables|Default|GetIsDissolving)
          (bind _output_get (Variables|Default|SetCurrentDissolveFraction (Math|Float|Lerp (Variables|Default|GetCurrentDissolveFraction) (Variables|Default|GetTargetDissolveFraction) (* (Utilities|Time|GetWorldDeltaSeconds) (/ 1.0 (Variables|Default|GetDissolveTime))))))
          (Rendering|Material|SetScalarParameterValueonMaterials (Variables|Default|GetMeshComponent) "DissolveFraction" _output_get)
          (if (Math|Float|NearlyEqual(Float) (Variables|Default|GetCurrentDissolveFraction) (Variables|Default|GetTargetDissolveFraction) 0.001)
            (Variables|Default|SetIsDissolving false))))
      (:then_1
        ;[1 1 1] Update emissive & edge thickness
        (if (and (Variables|Default|GetIsFlaringUp) (< (Variables|Default|GetFlareUpFraction) 1.0))
          (bind _output_get_2 (Variables|Default|SetFlareUpFraction (+ (Variables|Default|GetFlareUpFraction) (* (Utilities|Time|GetWorldDeltaSeconds) (/ 1.0 (Variables|Default|GetFlareUpTime))))))
          (Rendering|Material|SetScalarParameterValueonMaterials (Variables|Default|GetMeshComponent) "DissolveEmissiveAmount" (Math|Float|Lerp (Variables|Default|GetEmissiveAmountDefault) (Variables|Default|GetEmissiveAmountDissolving) (Math|Curves|GetFloatValue (Variables|Default|GetFlareCurve) _output_get_2)))
          (Rendering|Material|SetScalarParameterValueonMaterials (Variables|Default|GetMeshComponent) "DissolveEdgeThickness" (Math|Float|Lerp (Variables|Default|GetEdgeThicknessDefault) (Variables|Default|GetEdgeThicknessDissolving) (Math|Curves|GetFloatValue (Variables|Default|GetFlareCurve) (Variables|Default|GetFlareUpFraction))))
          (if (Math|Float|NearlyEqual(Float) (Variables|Default|GetFlareUpFraction) 1.0 0.001)
            (Variables|Default|SetIsFlaringUp false)))))))

(fn ActivateEffect
  (params (Fraction :type Float%20%28single-precision%29) (FlareUp :type Boolean))
  (Variables|Default|SetTargetDissolveFraction (Math|Float|Lerp (Variables|Default|GetMinFraction) (Variables|Default|GetMaxFraction) (- 1.0 Fraction)))
  (Variables|Default|SetFlareUpFraction 0.0)
  (Variables|Default|SetIsDissolving true)
  (Variables|Default|SetIsFlaringUp FlareUp))

(fn SetMesh
  (params (MeshComponent :type Mesh%20Component%20Object%20Reference))
  (Variables|Default|SetMeshComponent MeshComponent))

(fn FlareUp
  (Variables|Default|SetFlareUpFraction 0.0)
  (Variables|Default|SetIsFlaringUp true))